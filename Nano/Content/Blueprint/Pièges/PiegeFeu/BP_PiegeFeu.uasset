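; Fire trap Blueprint that cycles a Niagara wall of flames on and off.
; A Tick countdown, frame-based rather than timed, zeroes the particle velocities, then restores them after a delay.
; Construction script sets flame height from HauteurFlames, and a BeginPlay timeline animates that Z scale.
; Box overlap with BP_ThirdPersonCharacter only prints a hit message, with no damage applied.
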(event OnComponentBeginOverlap(Box)
  (params (OverlappedComponent :type Primitive%20Component%20Object%20Reference) (OtherActor :type Actor%20Object%20Reference) (OtherComp :type Primitive%20Component%20Object%20Reference) (OtherBodyIndex :type Integer) (bFromSweep :type Boolean) (SweepResult :type Hit%20Result%20Structure%20%28by%20ref%29))
  (Utilities|Casting|CastToBP_ThirdPersonCharacter OtherActor)
  (Development|PrintString "Hit Firewall"))

(event EventBeginPlay
  (Utilities|FlowControl|Sequence
    (:then_0
      (bind _scale (Timeline|Scale Play)
        (:Update
          (Transformation|SetRelativeScale3D (Variables|Default|GetScene) (Math|Vector|MakeVector 1.0 1.0 _scale))
          (Effects|Components|ParticleSystem|SetFloatParameter (Variables|Default|GetNiagara) "Velocity Max" 4e+02))))))

(event Collision|EventActorBeginOverlap
  (params (OtherActor :type Actor%20Object%20Reference)))

(event EventTick
  (params (DeltaSeconds :type Float%20%28single-precision%29))
  (bind _niagara (Variables|Default|GetNiagara))
  (bind _niagara_2 (Variables|Default|GetNiagara))
  (Variables|Default|SetSeconds (- (Variables|Default|GetSeconds) 1))
  (if (<= (Variables|Default|GetSeconds) 0)
    (Effects|Components|ParticleSystem|SetFloatParameter _niagara_2 "VelocityMin" 0.0)
    (Effects|Components|ParticleSystem|SetFloatParameter _niagara_2 "VelocityMax" 0.0)
    (Utilities|FlowControl|Delay 2e+01)
    (Variables|Default|SetSeconds 250)
    (Effects|Components|ParticleSystem|SetFloatParameter _niagara "VelocityMin" 1e+02)
    (Effects|Components|ParticleSystem|SetFloatParameter _niagara "VelocityMax" 4e+02)))

(fn ConstructionScript
  (Transformation|SetRelativeScale3D (Variables|Default|GetScene) (Math|Vector|MakeVector 1.0 1.0 (Variables|Default|GetHauteurFlames))))

(fn NewFunction0)