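; MurDestructible is a destructible wall, filed under traps, with a hit-point counter (PV).
; Each call to its Destruction event decrements PV by one, then destroys the actor when the count reaches zero or below.
; Debug strings print the remaining PV after a hit, or a death message when the wall is destroyed.
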(event EventDestruction
  ;[1 1 1] Voir si les PVs du mur est égale à 0. Si oui, le détruit
  (bind _result (Math|Integer|DecrementInt (Variables|HP|GetPV))
    (:%20%20
      (Variables|HP|SetPV _result)
      (if (<= (Variables|HP|GetPV) 0)
        ;[1 1 1] Destruction du mur
        (Actor|DestroyActor)
        (Development|PrintString "Dead!")
        (else
          (Development|PrintString (Utilities|String|Append "PV Mur:" (Utilities|String|ToString(Integer) (Variables|HP|GetPV))) true true "(R=0.000000,G=0.660000,B=1.000000,A=1.000000)" 1.0))))))

(fn ConstructionScript)