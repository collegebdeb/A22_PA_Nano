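; BP_PieceVaisseauParent is the parent Blueprint for collectible ship parts that the player picks up by touching them.
; It caches the player's BP_ThirdPersonCharacter on BeginPlay and compares it with any actor entering its Sphere.
; On a match, it passes IndexPart to the character through the PickUpVaisseauMessage interface call for the on-screen pickup display, then destroys itself.
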(event OnComponentBeginOverlap(Sphere)
  (params (OverlappedComponent :type Primitive%20Component%20Object%20Reference) (OtherActor :type Actor%20Object%20Reference) (OtherComp :type Primitive%20Component%20Object%20Reference) (OtherBodyIndex :type Integer) (bFromSweep :type Boolean) (SweepResult :type Hit%20Result%20Structure%20%28by%20ref%29))
  ;[1 1 1] Si le personnage touche le pickUp
  (if (== OtherActor (Variables|Reference|GetAs%20BP%20Third%20Person%20Character))
    ;[1 1 1] Blueprint Interface pour afficher à l'écran si l'objet est récupéré
    (Class|BPIPickUp|PickUpVaisseau(Message) (Variables|Reference|GetAs%20BP%20Third%20Person%20Character) (Variables|NumeroPart|GetIndexPart))
    ;[1 1 1] Détruire l'actor
    (Actor|DestroyActor)))

(event EventBeginPlay
  ;[1 1 1] Caster une référence du personnage
  (bind _asbp_third_person_character (Utilities|Casting|CastToBP_ThirdPersonCharacter (Game|GetPlayerCharacter 0)))
  (Variables|Reference|SetAs%20BP%20Third%20Person%20Character _asbp_third_person_character))

(fn ConstructionScript)