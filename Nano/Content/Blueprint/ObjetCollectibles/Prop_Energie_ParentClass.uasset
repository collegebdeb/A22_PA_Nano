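; Parent Blueprint for energy collectibles that refill the player's energy gauge on pickup.
; A looping timeline alternates between play and reverse to bob the prop up and down by an interval.
; When the cached player character overlaps the capsule, the object destroys itself and passes its energy value to RecevoirBonusEnergie.
; The construction script tints the prop through a dynamic oxygen-tank material instance.
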(event OnComponentBeginOverlap(Capsule)
  (params (OverlappedComponent :type Primitive%20Component%20Object%20Reference) (OtherActor :type Actor%20Object%20Reference) (OtherComp :type Primitive%20Component%20Object%20Reference) (OtherBodyIndex :type Integer) (bFromSweep :type Boolean) (SweepResult :type Hit%20Result%20Structure%20%28by%20ref%29))
  (bind _as_bp_third_person_character (Variables|Reference|GetAs%20BP%20Third%20Person%20Character))
  ;[1 1 1] Voir si l'élément qui entre dans la collision de l'objet est le joueur
  (if (== OtherActor _as_bp_third_person_character)
    (Utilities|FlowControl|Sequence
      (:then_0
        ;[1 1 1] Détruit l'objet
        (Actor|DestroyActor))
      (:then_1
        ;[1 1 1] Remplir la jauge du joueur
        (Default|RecevoirBonusEnergie _as_bp_third_person_character (Variables|Energie|GetValeurEnergie))))))

(event Custom|Reverse
  (bind _props (Variables|Default|GetProps))
  (bind _relativelocation (Variables|/Script/Engine.SceneComponent|GetRelativeLocation _props))
  (bind _newtrack_0 (Timeline|LerpAnimationHautBas Reverse)
    (:Update
      (Transformation|SetRelativeLocation (Variables|Default|GetProps) (Math|Vector|MakeVector (.x _relativelocation) (.y _relativelocation) (Math|Float|Lerp 0.0 (+ (.z _relativelocation) (Variables|Default|GetIntervalle)) _newtrack_0)) false false))
    (:Finished
      (if (Variables|Default|GetIsFromStart?)
        (Variables|Default|SetIsFromStart? false)
        (CallFunction|Reverse)
        (else
          (Variables|Default|SetIsFromStart? true)
          (CallFunction|Recommencer))))))

(event Custom|Recommencer
  (bind _props (Variables|Default|GetProps))
  (bind _relativelocation (Variables|/Script/Engine.SceneComponent|GetRelativeLocation _props))
  (bind _newtrack_0 (Timeline|LerpAnimationHautBas Play)
    (:Update
      (Transformation|SetRelativeLocation (Variables|Default|GetProps) (Math|Vector|MakeVector (.x _relativelocation) (.y _relativelocation) (Math|Float|Lerp 0.0 (+ (.z _relativelocation) (Variables|Default|GetIntervalle)) _newtrack_0)) false false))
    (:Finished
      (if (Variables|Default|GetIsFromStart?)
        (Variables|Default|SetIsFromStart? false)
        (CallFunction|Reverse)
        (else
          (Variables|Default|SetIsFromStart? true)
          (CallFunction|Recommencer))))))

(event EventBeginPlay
  (bind _props (Variables|Default|GetProps))
  (bind _relativelocation (Variables|/Script/Engine.SceneComponent|GetRelativeLocation _props))
  ;[1 1 1] Prendre en référence le joueur
  (Utilities|FlowControl|Sequence
    (:then_0
      (bind _asbp_third_person_character (Utilities|Casting|CastToBP_ThirdPersonCharacter (Game|GetPlayerCharacter 0)))
      (Variables|Reference|SetAs%20BP%20Third%20Person%20Character _asbp_third_person_character))
    (:then_1
      (bind _newtrack_0 (Timeline|LerpAnimationHautBas Play)
        (:Update
          (Transformation|SetRelativeLocation (Variables|Default|GetProps) (Math|Vector|MakeVector (.x _relativelocation) (.y _relativelocation) (Math|Float|Lerp 0.0 (+ (.z _relativelocation) (Variables|Default|GetIntervalle)) _newtrack_0)) false false))
        (:Finished
          (if (Variables|Default|GetIsFromStart?)
            (Variables|Default|SetIsFromStart? false)
            (CallFunction|Reverse)
            (else
              (Variables|Default|SetIsFromStart? true)
              (CallFunction|Recommencer))))))))

(fn ConstructionScript
  (bind _returnvalue (Rendering|Material|CreateDynamicMaterialInstance (Variables|Default|GetProps) 0 "/Game/Assets/Collectible/M_OxygenTank.M_OxygenTank" "None" :!class /Script/Engine.PrimitiveComponent))
  (bind _output_get (Variables|Default|SetMateriel_Ref _returnvalue))
  (Rendering|Material|SetVectorParameterValue _output_get "CouleurOverwrite" (Variables|Default|GetCouleur) :!class /Script/Engine.MaterialInstanceDynamic))