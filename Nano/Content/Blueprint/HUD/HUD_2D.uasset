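; 2D HUD Blueprint that shows the in-game UI and manages the pause, death and success menus.
; The death menu fades in over a timeline, hiding the HUD, then pauses the game; the pause menu pauses immediately.
; Tick caches the player character and recolors menu buttons by keyboard focus.
; The success event fades in its menu, disables player input and movement, then quits the game after a short delay.
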(event Custom|ApparitionMenuPause
  (Utilities|IsValid (Variables|Reference|GetMenuPause)
    (:Is%20Valid
      _)
    (:Is%20Not%20Valid
      (bind _returnvalue (Game|ConstructObjectfromClass "/Game/Blueprint/HUD/WB_MenuPause.WB_MenuPause_C"))
      (bind _output_get (Variables|Reference|SetMenuPause _returnvalue))))
  (Input|SetInputModeUIOnly (Game|GetPlayerController 0) _output_get "DoNotLock")
  (UserInterface|Viewport|AddtoViewport _output_get 0)
  (Variables|Default|SetSetArray (Variables|/Game/Blueprint/HUD/WB_MenuPause.WB_MenuPause_C|GetArray _output_get))
  (Game|SetGamePaused true))

(event Custom|Event_MenuReussite
  (bind _as_bp_third_person_character (Variables|Reference|GetAs%20BP%20Third%20Person%20Character))
  (bind _newtrack_0 (Timeline|Timeline_0 Play)
    (:Update
      (Widget|SetRenderOpacity (Variables|Reference|GetMenuReussite) _newtrack_0)
      (Input|DisableInput _as_bp_third_person_character 0)
      (Pawn|Components|CharacterMovement|DisableMovement (Variables|/Script/Engine.Character|GetCharacterMovement _as_bp_third_person_character)))
    (:Finished
      (Utilities|FlowControl|Delay 1.5)
      (Game|QuitGame 0 "Quit" false))))

(event Custom|DisparitionMenuPause
  (bind _menupause (Variables|Reference|GetMenuPause))
  (Utilities|IsValid _menupause
    (:Is%20Valid
      (Widget|RemovefromParent _menupause)
      (Game|SetGamePaused false))))

(event Custom|MortMenu
  (bind _returnvalue (Game|ConstructObjectfromClass "/Game/Blueprint/HUD/WB_MenuMort.WB_MenuMort_C"))
  (bind _output_get (Variables|Reference|SetMenuMort _returnvalue))
  (Utilities|FlowControl|Sequence
    (:then_0
      (Widget|SetRenderOpacity _output_get 0.0))
    (:then_1
      (UserInterface|Viewport|AddtoViewport _output_get 0)
      (Components|Timeline|SetPlayRate (Variables|Default|GetApparitionMenuMort) (/ 1.0 (Variables|Default|GetTempsTimelineMort)))
      (Widget|SetRenderOpacity (Variables|Reference|GetUI_Reference) 0.0)
      (Variables|Default|SetSetArray (Variables|/Game/Blueprint/HUD/WB_MenuMort.WB_MenuMort_C|GetArray (Variables|Reference|GetMenuMort)))
      (bind _newtrack_0 (Timeline|ApparitionMenuMort Play)
        (:Update
          (Widget|SetRenderOpacity (Variables|Reference|GetMenuMort) (Math|Float|Lerp 0.0 1.0 _newtrack_0)))
        (:Finished
          (Input|SetInputModeUIOnly (Game|GetPlayerController 0) 0 "DoNotLock")
          (Class|Actor|SetTickablewhenPaused true)
          (Game|SetGamePaused true))))))

(event Custom|UpdateButton
  (for _array_element (Variables|Default|GetSetArray)
    (if (Class|Widget|HasKeyboardFocus _array_element)
      (Class|Button|SetBackgroundColor _array_element "(R=0.479167,G=0.155250,B=0.000000,A=1.000000)")
      (else
        (Class|Button|SetBackgroundColor _array_element "(R=0.219510,G=0.354167,B=0.277443,A=1.000000)")))))

(event EventBeginPlay
  (bind _returnvalue (Game|ConstructObjectfromClass "/Game/Blueprint/HUD/WB_HUD.WB_HUD_C"))
  (bind _output_get (Variables|Reference|SetUI_Reference _returnvalue))
  (UserInterface|Viewport|AddtoViewport _output_get 0))

(event EventTick
  (params (DeltaSeconds :type Float%20%28single-precision%29))
  (Utilities|FlowControl|Sequence
    (:then_0
      ;[1 1 1] Update constamment le Player Controller
      (bind _asbp_third_person_character (Utilities|Casting|CastToBP_ThirdPersonCharacter (Game|GetPlayerCharacter 0)))
      (Variables|Reference|SetAs%20BP%20Third%20Person%20Character _asbp_third_person_character))
    (:then_1
      (Utilities|IsValid (Variables|Reference|GetMenuMort)
        (:Is%20Valid
          _)
        (:Is%20Not%20Valid
          (Utilities|IsValid (Variables|Reference|GetMenuPause)
            (:Is%20Valid
              _))))
      (CallFunction|UpdateButton))))

(fn ConstructionScript)