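; Trap actor that repeatedly spawns a meteorite at its Spawner component and moves it in a straight line.
; A timeline lerps the meteorite along world X from the trap's root by the scaled arrow length, printing each position for debug.
; When the timeline finishes, the meteorite is destroyed and respawned after a short delay, looping indefinitely.
; The construction script applies the editable Spawner pitch and direction arrow length.
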(event Custom|DestroyMeteorite
  (Actor|DestroyActor (Variables|Default|GetNewVar_0))
  (Utilities|FlowControl|Delay 2.0)
  (CallFunction|RespawnObject))

(event Custom|RespawnObject
  (bind _defaultsceneroot (Variables|Default|GetDefaultSceneRoot))
  (bind _returnvalue (Transformation|GetWorldLocation _defaultsceneroot))
  (bind _output_get1 (CallFunction|NewFunction0))
  (bind _newtrack_0 (Timeline|Timeline_0 PlayFromStart)
    (:Update
      (Development|PrintString (Utilities|String|ToString(Vector) (Math|Vector|MakeVector (Math|Float|Lerp (.x _returnvalue) (+ (.x _returnvalue) (* (Variables|Default|GetArrow%20Length) (Variables|/Script/Engine.ArrowComponent|GetArrowSize (Variables|Default|GetDirectionMeteoriteTombee)))) _newtrack_0) (.y _returnvalue) (.z _returnvalue))) true true "(R=0.000000,G=0.660000,B=1.000000,A=1.000000)" 0.1)
      (Transformation|SetRelativeLocation (Variables|/Script/Engine.Actor|GetRootComponent _output_get1) (Math|Vector|MakeVector (Math|Float|Lerp (.x _returnvalue) (+ (.x _returnvalue) (* (Variables|Default|GetArrow%20Length) (Variables|/Script/Engine.ArrowComponent|GetArrowSize (Variables|Default|GetDirectionMeteoriteTombee)))) _newtrack_0) (.y _returnvalue) (.z _returnvalue)) false false))
    (:Finished
      (CallFunction|DestroyMeteorite))))

(event EventBeginPlay
  (bind _defaultsceneroot (Variables|Default|GetDefaultSceneRoot))
  (bind _returnvalue (Transformation|GetWorldLocation _defaultsceneroot))
  (bind _output_get1 (CallFunction|NewFunction0))
  (bind _newtrack_0 (Timeline|Timeline_0 PlayFromStart)
    (:Update
      (Development|PrintString (Utilities|String|ToString(Vector) (Math|Vector|MakeVector (Math|Float|Lerp (.x _returnvalue) (+ (.x _returnvalue) (* (Variables|Default|GetArrow%20Length) (Variables|/Script/Engine.ArrowComponent|GetArrowSize (Variables|Default|GetDirectionMeteoriteTombee)))) _newtrack_0) (.y _returnvalue) (.z _returnvalue))) true true "(R=0.000000,G=0.660000,B=1.000000,A=1.000000)" 0.1)
      (Transformation|SetRelativeLocation (Variables|/Script/Engine.Actor|GetRootComponent _output_get1) (Math|Vector|MakeVector (Math|Float|Lerp (.x _returnvalue) (+ (.x _returnvalue) (* (Variables|Default|GetArrow%20Length) (Variables|/Script/Engine.ArrowComponent|GetArrowSize (Variables|Default|GetDirectionMeteoriteTombee)))) _newtrack_0) (.y _returnvalue) (.z _returnvalue)) false false))
    (:Finished
      (CallFunction|DestroyMeteorite))))

(fn ConstructionScript
  (bind _spawner (Variables|Default|GetSpawner))
  (bind _relativerotation (Variables|/Script/Engine.SceneComponent|GetRelativeRotation _spawner))
  (Utilities|FlowControl|Sequence
    (:then_0
      (Transformation|SetRelativeRotation (Variables|Default|GetSpawner) (Math|Rotator|MakeRotator (.roll _relativerotation) (Variables|Default|GetRotationPositionMeteorite) (.yaw _relativerotation)) false false))
    (:then_1
      (Variables|/Script/Engine.ArrowComponent|SetArrowLength (Variables|Default|GetDirectionMeteoriteTombee) (Variables|Default|GetArrow%20Length)))))

(fn NewFunction0
  (bind _returnvalue (Game|SpawnActorfromClass "/Game/Blueprint/Pièges/BP_Meteorite.BP_Meteorite_C" (Transformation|GetWorldTransform (Variables|Default|GetSpawner)) "Undefined" 0 0))
  (bind _output_get (Variables|Default|SetNewVar_0 _returnvalue))
  (return _output_get))