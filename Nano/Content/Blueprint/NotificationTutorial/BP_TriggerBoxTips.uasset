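; Tutorial tip trigger box that shows a WG_Notification widget with configurable text when the player character overlaps it.
; The first entry shows the tip immediately; later, Tick shows it again after three seconds inside without an existing widget.
; An Opacity timeline fades the widget in, then reverses on exit and removes it once finished.
; DoOnce gates prevent repeat triggers, with the delayed one reset on exit.
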(event Custom|Disparition
  ;[1 1 1] Animation lorsque le joueur quitte le triggerbox
  ;[1 1 1] Animation et Lerp de l'opacity du widget pour un fade-in/fade-out
  ;;[1 1 1] Set l'opacity selon si le joueur entre, quitte ou attends pendant un temps dans le triggerbox
  (bind _newtrack_0 (Timeline|Opacity Reverse)
    (:Update
      (Widget|SetRenderOpacity (Variables|Default|GetWidget_Ref) (Math|Float|Lerp 0.0 1.0 _newtrack_0)))
    (:Finished
      ;;[1 1 1] Si l'animation est complétée, enlève le widget et set à faux le booléen pour si cet élément n'existe pas
      (if (not (Variables|Default|GetIsIn?))
        (Variables|Default|SetWidgetIsExisting? false)
        (Widget|RemovefromParent (Variables|Default|GetWidget_Ref))))))

(event Custom|NotifApresTemps
  ;[1 1 1] Créer le widget après un timer si le joueur est coincé
  ;[1 1 1] Création et affichage initiale du widget lorsque le triggerbox overlap avec le joueur ou celui-ci attends un certain temps
  ;;[1 1 1] Créer le widget, changer le texte à l'intérieur et change le texte existant avec celui modifier dans le triggerbox
  (bind _returnvalue (UserInterface|CreateWidget "/Game/Blueprint/NotificationTutorial/WG_Notification.WG_Notification_C" (Game|GetPlayerController 0)))
  (Variables|Default|SetWidgetIsExisting? true)
  (bind _output_get (Variables|Default|SetWidget_Ref _returnvalue))
  (Variables|/Game/Blueprint/NotificationTutorial/WG_Notification.WG_Notification_C|SetTextNotification _output_get (Variables|Default|GetText))
  ;;[1 1 1] Mettre le widget dans le viewport du joueur. Mettre l'opacity à 0
  (UserInterface|Viewport|AddtoViewport (Variables|Default|GetWidget_Ref) 0)
  (Widget|SetRenderOpacity (Variables|Default|GetWidget_Ref) 0.0)
  ;[1 1 1] Animation et Lerp de l'opacity du widget pour un fade-in/fade-out
  ;;[1 1 1] Set l'opacity selon si le joueur entre, quitte ou attends pendant un temps dans le triggerbox
  (bind _newtrack_0 (Timeline|Opacity PlayFromStart)
    (:Update
      (Widget|SetRenderOpacity (Variables|Default|GetWidget_Ref) (Math|Float|Lerp 0.0 1.0 _newtrack_0)))
    (:Finished
      ;;[1 1 1] Si l'animation est complétée, enlève le widget et set à faux le booléen pour si cet élément n'existe pas
      (if (not (Variables|Default|GetIsIn?))
        (Variables|Default|SetWidgetIsExisting? false)
        (Widget|RemovefromParent (Variables|Default|GetWidget_Ref))))))

(event Collision|EventActorBeginOverlap
  (params (OtherActor :type Actor%20Object%20Reference))
  ;[1 1 1] Événement qui arrive lorsque le joueur entre dans le triggerbox
  ;;[1 1 1] Voir si le joueur overlap le triggerbox
  (if (== OtherActor (Variables|Default|GetAs%20BP%20Third%20Person%20Character))
    ;;[1 1 1] Jouer à l'intérieur du triggerbox (fait une seule fois)
    (Variables|Default|SetIsIn? true)
    (Utilities|FlowControl|DoOnce false
      (:Completed
        ;[1 1 1] Création et affichage initiale du widget lorsque le triggerbox overlap avec le joueur ou celui-ci attends un certain temps
        ;;[1 1 1] Créer le widget, changer le texte à l'intérieur et change le texte existant avec celui modifier dans le triggerbox
        (bind _returnvalue (UserInterface|CreateWidget "/Game/Blueprint/NotificationTutorial/WG_Notification.WG_Notification_C" (Game|GetPlayerController 0)))
        (Variables|Default|SetWidgetIsExisting? true)
        (bind _output_get (Variables|Default|SetWidget_Ref _returnvalue))
        (Variables|/Game/Blueprint/NotificationTutorial/WG_Notification.WG_Notification_C|SetTextNotification _output_get (Variables|Default|GetText))
        ;;[1 1 1] Mettre le widget dans le viewport du joueur. Mettre l'opacity à 0
        (UserInterface|Viewport|AddtoViewport (Variables|Default|GetWidget_Ref) 0)
        (Widget|SetRenderOpacity (Variables|Default|GetWidget_Ref) 0.0)
        ;[1 1 1] Animation et Lerp de l'opacity du widget pour un fade-in/fade-out
        ;;[1 1 1] Set l'opacity selon si le joueur entre, quitte ou attends pendant un temps dans le triggerbox
        (bind _newtrack_0 (Timeline|Opacity PlayFromStart)
          (:Update
            (Widget|SetRenderOpacity (Variables|Default|GetWidget_Ref) (Math|Float|Lerp 0.0 1.0 _newtrack_0)))
          (:Finished
            ;;[1 1 1] Si l'animation est complétée, enlève le widget et set à faux le booléen pour si cet élément n'existe pas
            (if (not (Variables|Default|GetIsIn?))
              (Variables|Default|SetWidgetIsExisting? false)
              (Widget|RemovefromParent (Variables|Default|GetWidget_Ref)))))))))

(event EventBeginPlay
  ;[1 1 1] Caster le joueur comme référence de collision possible avec le triggerbox
  (bind _asbp_third_person_character (Utilities|Casting|CastToBP_ThirdPersonCharacter (Game|GetPlayerCharacter 0)))
  (Variables|Default|SetAs%20BP%20Third%20Person%20Character _asbp_third_person_character))

(event Collision|EventActorEndOverlap
  (params (OtherActor :type Actor%20Object%20Reference))
  ;[1 1 1] Événement qui arrive lorsque le joueur quitte la zone
  (if (== OtherActor (Variables|Default|GetAs%20BP%20Third%20Person%20Character))
    (Variables|Default|SetIsIn? false)
    (CallFunction|Disparition)
    ;[1 1 1] Si le joueur atteint un temps, la notification apparaît
    (Utilities|FlowControl|DoOnce false) ; enters at Reset
  ))

(event EventTick
  (params (DeltaSeconds :type Float%20%28single-precision%29))
  ;[1 1 1] Voir si le joueur est dans le triggerbox sans avoir le widget d'existant
  (if (and (Variables|Default|GetIsIn?) (not (Variables|Default|GetWidgetIsExisting?)))
    ;[1 1 1] Si le joueur atteint un temps, la notification apparaît
    (bind _output_get (Variables|Default|SetTimeInterieur (+ DeltaSeconds (Variables|Default|GetTimeInterieur))))
    (if (>= _output_get 3.0)
      (Utilities|FlowControl|DoOnce false
        (:Completed
          (CallFunction|NotifApresTemps)
          ;[1 1 1] Mets le compteur à 0
          (Variables|Default|SetTimeInterieur 0.0 :!label _label))))
    (else
      (goto _label))))

(fn ConstructionScript)