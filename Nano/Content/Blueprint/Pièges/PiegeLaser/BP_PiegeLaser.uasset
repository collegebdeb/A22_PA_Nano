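; Laser trap that slides back and forth along a trail between Start and End, killing the player on contact.
; The construction script sizes the trail from DistanceParcourue and places the emitter at the end matching IsReversed.
; A timeline lerps the emitter while line traces set Niagara beam length, place impact sparks or trigger burn effects and player death.
; At each end it pauses before reversing, with a looping timer keeping the trace running.
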(event Custom|FinirDeplacement
  ;[0.1206 0 1] Lorsque le timeline finit, effectue un Delay selon une variable et inverse le boolean selon le résultat précédent
  (Utilities|FlowControl|Sequence
    (:then_0
      ;[0 0.9597 1] Lorsque le laser est immobile
      ;;[1 1 1] Le son est désactivé
      (Utilities|FlowControl|DoOnce false) ; enters at Reset
    )
    (:then_1
      ;;[1 1 1] Set un timer (tick personnalisé)
      (bind _returnvalue (Utilities|Time|SetTimerbyEvent (delegate Custom|LinetracePause) (/ 1.0 15.0) true))
      ;;[1 1 1] Pause du laser
      (Utilities|FlowControl|Delay (Variables|Laser|GetPause%20Laser))
      ;;[1 1 1] Changement de mode
      (if (Variables|ModeLaser|GetIsReversed?)
        (Utilities|Time|ClearandInvalidateTimerbyHandle _returnvalue)
        (Variables|ModeLaser|SetIsReversed? false)
        (CallFunction|AnimationNormal)
        (else
          (Utilities|Time|ClearandInvalidateTimerbyHandle _returnvalue)
          (Variables|ModeLaser|SetIsReversed? true)
          (CallFunction|Inverse))))))

(event Custom|Inverse
  (bind _start (Variables|Default|GetStart))
  (bind _end (Variables|Default|GetEnd))
  (bind _as_bp_third_person_character (Variables|Reference|GetAs%20BP%20Third%20Person%20Character))
  (bind _as_bp_third_person_character_2 (Variables|Reference|GetAs%20BP%20Third%20Person%20Character))
  (bind _spark (Variables|Default|GetSpark))
  (bind _spark_2 (Variables|Default|GetSpark))
  (bind _sphere (Variables|Default|GetSphere))
  (bind _ns_piegelaser (Variables|Default|GetNS_PiegeLaser))
  (bind _returnvalue (Transformation|GetWorldLocation _end))
  (bind _returnvalue_2 (Transformation|GetWorldLocation _start))
  (bind _returnvalue_3 (Transformation|GetWorldLocation _sphere))
  (bind _lasermort (Variables|/Game/ThirdPerson/Blueprints/BP_ThirdPersonCharacter.BP_ThirdPersonCharacter_C|GetLaserMort _as_bp_third_person_character_2))
  ;[1 0 0] Update la location du laser selon un timeline
  (Components|Activation|Activate (Variables|Default|GetSonPiegeLaser) false)
  ;;[1 1 1] Prendre l'alpha du timeline pour l'utiliser pour un Lerp
  (bind _newtrack_0 (Timeline|Timeline_0 ReverseFromEnd)
    (:Update
      (Transformation|SetWorldLocation (Variables|Default|GetSphere) (Math|Vector|Lerp(Vector) (Math|Vector|MakeVector (.x _returnvalue_2) (.y _returnvalue_2) (+ (Variables|Mesh|GetOffsetMesh) (.z _returnvalue_2))) (Math|Vector|MakeVector (.x _returnvalue) (.y _returnvalue) (+ (Variables|Mesh|GetOffsetMesh) (.z _returnvalue))) _newtrack_0) false false)
      ;[0 0.1828 1] Calcul de la position et longueur du linetrace à chaque frame
      ;;[1 1 1] Créer un linetrace selon la position update du Lerp et vers les axes des Z
      (bind _outhit (Collision|LineTraceByChannel (Math|Vector|MakeVector (.x _returnvalue_3) (.y _returnvalue_3) (.z _returnvalue_3)) (+ (Transformation|GetWorldLocation (Variables|Default|GetSphere)) (* (Math|Vector|GetUpVector (Variables|Default|GetDefaultSceneRoot)) (Variables|Laser|GetPorteeMaximaleLaser))) "TraceTypeQuery3" false 0 "None"))
      ;[0.1077 0 1] Si le laser touche le joueur
      ;;[1 1 1] Voir si le laser touche le personnage (BP_ThirdPersonCharacter)
      (if (== _as_bp_third_person_character (.HitActor (Collision|BreakHitResult _outhit))) ; Voir si le laser touche le joueur
        (Components|Timeline|SetPlayRate (Variables|Default|GetTimeline_2) 0.2)
        (bind _opacitymaskvisibility (Timeline|Timeline_2 Play)
          (:Update
            (Rendering|Material|SetScalarParameterValue (Variables|/Game/ThirdPerson/Blueprints/BP_ThirdPersonCharacter.BP_ThirdPersonCharacter_C|GetMaterialBrulure _as_bp_third_person_character) "Visibility" (Math|Float|Lerp 0.0 2.0 _opacitymaskvisibility) :!class /Script/Engine.MaterialInstanceDynamic)
            ;[0 0.3378 1] Effet lors la mort du personnage
            (Effects|Components|ParticleSystem|SetFloatParameter _lasermort "SpawnParticules" 1.0)
            ;;[1 1 1] Lerp de l'apparition des particules
            (bind _newtrack_0_2 (Timeline|DisparitionParticule PlayFromStart)
              (:Update
                (Effects|Components|ParticleSystem|SetFloatParameter _lasermort "SpawnRate" (Math|Float|Lerp 5e+03 0.0 _newtrack_0_2))
                (CallFunction|MortPerso) ; Tue le personnage
              ))))
        (else
          ;[1 1 1] Selon si le laser touche une surface, change la taille du laser proportionnellement selon la location de l'impact
          (if (.bBlockingHit (Collision|BreakHitResult _outhit))
            (Niagara|SetNiagaraVariable(Vector3) _ns_piegelaser "BeamEnd" (Math|Vector|MakeVector 0.0 0.0 (.Distance (Collision|BreakHitResult _outhit))))
            ;[1 1 1] Mettre à la place de l'impact le VFX d'étincelle
            (Components|Activation|Activate _spark_2 false)
            (Niagara|SetNiagaraVariable(Float) _spark_2 "BeamSpawnProb" 1.0)
            (Transformation|SetWorldLocation _spark_2 (.Location (Collision|BreakHitResult _outhit)) false false)
            (else
              (Niagara|SetNiagaraVariable(Vector3) _ns_piegelaser "BeamEnd" (Math|Vector|MakeVector 0.0 0.0 (Variables|Laser|GetPorteeMaximaleLaser)))
              (Components|Activation|Deactivate _spark)
              (Niagara|SetNiagaraVariable(Float) _spark "BeamSpawnProb" 0.0))))))
    (:Finished
      ;;[1 1 1] Lorsque la timeline est finalisé
      (CallFunction|FinirDeplacement))))

(event Custom|MortPerso
  ;[1 1 1] Si le joueur touche le laser, celui-ci appelle la condition de mort
  (Default|Destroy (Variables|Reference|GetAs%20BP%20Third%20Person%20Character) "" "un piège laser"))

(event Custom|AnimationNormal
  (bind _start (Variables|Default|GetStart))
  (bind _end (Variables|Default|GetEnd))
  (bind _as_bp_third_person_character (Variables|Reference|GetAs%20BP%20Third%20Person%20Character))
  (bind _as_bp_third_person_character_2 (Variables|Reference|GetAs%20BP%20Third%20Person%20Character))
  (bind _spark (Variables|Default|GetSpark))
  (bind _spark_2 (Variables|Default|GetSpark))
  (bind _sphere (Variables|Default|GetSphere))
  (bind _ns_piegelaser (Variables|Default|GetNS_PiegeLaser))
  (bind _returnvalue (Transformation|GetWorldLocation _end))
  (bind _returnvalue_2 (Transformation|GetWorldLocation _start))
  (bind _returnvalue_3 (Transformation|GetWorldLocation _sphere))
  (bind _lasermort (Variables|/Game/ThirdPerson/Blueprints/BP_ThirdPersonCharacter.BP_ThirdPersonCharacter_C|GetLaserMort _as_bp_third_person_character_2))
  ;[1 0 0] Update la location du laser selon un timeline
  (Components|Activation|Activate (Variables|Default|GetSonPiegeLaser) false)
  ;;[1 1 1] Prendre l'alpha du timeline pour l'utiliser pour un Lerp
  (bind _newtrack_0 (Timeline|Timeline_0 Play)
    (:Update
      (Transformation|SetWorldLocation (Variables|Default|GetSphere) (Math|Vector|Lerp(Vector) (Math|Vector|MakeVector (.x _returnvalue_2) (.y _returnvalue_2) (+ (Variables|Mesh|GetOffsetMesh) (.z _returnvalue_2))) (Math|Vector|MakeVector (.x _returnvalue) (.y _returnvalue) (+ (Variables|Mesh|GetOffsetMesh) (.z _returnvalue))) _newtrack_0) false false)
      ;[0 0.1828 1] Calcul de la position et longueur du linetrace à chaque frame
      ;;[1 1 1] Créer un linetrace selon la position update du Lerp et vers les axes des Z
      (bind _outhit (Collision|LineTraceByChannel (Math|Vector|MakeVector (.x _returnvalue_3) (.y _returnvalue_3) (.z _returnvalue_3)) (+ (Transformation|GetWorldLocation (Variables|Default|GetSphere)) (* (Math|Vector|GetUpVector (Variables|Default|GetDefaultSceneRoot)) (Variables|Laser|GetPorteeMaximaleLaser))) "TraceTypeQuery3" false 0 "None"))
      ;[0.1077 0 1] Si le laser touche le joueur
      ;;[1 1 1] Voir si le laser touche le personnage (BP_ThirdPersonCharacter)
      (if (== _as_bp_third_person_character (.HitActor (Collision|BreakHitResult _outhit))) ; Voir si le laser touche le joueur
        (Components|Timeline|SetPlayRate (Variables|Default|GetTimeline_2) 0.2)
        (bind _opacitymaskvisibility (Timeline|Timeline_2 Play)
          (:Update
            (Rendering|Material|SetScalarParameterValue (Variables|/Game/ThirdPerson/Blueprints/BP_ThirdPersonCharacter.BP_ThirdPersonCharacter_C|GetMaterialBrulure _as_bp_third_person_character) "Visibility" (Math|Float|Lerp 0.0 2.0 _opacitymaskvisibility) :!class /Script/Engine.MaterialInstanceDynamic)
            ;[0 0.3378 1] Effet lors la mort du personnage
            (Effects|Components|ParticleSystem|SetFloatParameter _lasermort "SpawnParticules" 1.0)
            ;;[1 1 1] Lerp de l'apparition des particules
            (bind _newtrack_0_2 (Timeline|DisparitionParticule PlayFromStart)
              (:Update
                (Effects|Components|ParticleSystem|SetFloatParameter _lasermort "SpawnRate" (Math|Float|Lerp 5e+03 0.0 _newtrack_0_2))
                (CallFunction|MortPerso) ; Tue le personnage
              ))))
        (else
          ;[1 1 1] Selon si le laser touche une surface, change la taille du laser proportionnellement selon la location de l'impact
          (if (.bBlockingHit (Collision|BreakHitResult _outhit))
            (Niagara|SetNiagaraVariable(Vector3) _ns_piegelaser "BeamEnd" (Math|Vector|MakeVector 0.0 0.0 (.Distance (Collision|BreakHitResult _outhit))))
            ;[1 1 1] Mettre à la place de l'impact le VFX d'étincelle
            (Components|Activation|Activate _spark_2 false)
            (Niagara|SetNiagaraVariable(Float) _spark_2 "BeamSpawnProb" 1.0)
            (Transformation|SetWorldLocation _spark_2 (.Location (Collision|BreakHitResult _outhit)) false false)
            (else
              (Niagara|SetNiagaraVariable(Vector3) _ns_piegelaser "BeamEnd" (Math|Vector|MakeVector 0.0 0.0 (Variables|Laser|GetPorteeMaximaleLaser)))
              (Components|Activation|Deactivate _spark)
              (Niagara|SetNiagaraVariable(Float) _spark "BeamSpawnProb" 0.0))))))
    (:Finished
      ;;[1 1 1] Lorsque la timeline est finalisé
      (CallFunction|FinirDeplacement))))

(event Custom|LinetracePause
  ;[0 0.9597 1] Lorsque le laser est immobile
  (Utilities|FlowControl|Sequence
    (:then_0
      ;;[1 1 1] Le son est désactivé
      (Utilities|FlowControl|DoOnce false
        (:Completed
          (Components|Activation|Deactivate (Variables|Default|GetSonPiegeLaser)))))
    (:then_1
      (CallFunction|LaserContinuePause) ; Projeter le linetrace
    )))

(event Custom|LaserContinuePause
  (bind _as_bp_third_person_character (Variables|Reference|GetAs%20BP%20Third%20Person%20Character))
  (bind _as_bp_third_person_character_2 (Variables|Reference|GetAs%20BP%20Third%20Person%20Character))
  (bind _spark (Variables|Default|GetSpark))
  (bind _spark_2 (Variables|Default|GetSpark))
  (bind _sphere (Variables|Default|GetSphere))
  (bind _ns_piegelaser (Variables|Default|GetNS_PiegeLaser))
  (bind _returnvalue (Transformation|GetWorldLocation _sphere))
  (bind _lasermort (Variables|/Game/ThirdPerson/Blueprints/BP_ThirdPersonCharacter.BP_ThirdPersonCharacter_C|GetLaserMort _as_bp_third_person_character_2))
  ;[0 0.1828 1] Calcul de la position et longueur du linetrace à chaque frame
  ;;[1 1 1] Créer un linetrace selon la position update du Lerp et vers les axes des Z
  (bind _outhit (Collision|LineTraceByChannel (Math|Vector|MakeVector (.x _returnvalue) (.y _returnvalue) (.z _returnvalue)) (+ (Transformation|GetWorldLocation (Variables|Default|GetSphere)) (* (Math|Vector|GetUpVector (Variables|Default|GetDefaultSceneRoot)) (Variables|Laser|GetPorteeMaximaleLaser))) "TraceTypeQuery3" false 0 "None"))
  ;[0.1077 0 1] Si le laser touche le joueur
  ;;[1 1 1] Voir si le laser touche le personnage (BP_ThirdPersonCharacter)
  (if (== _as_bp_third_person_character (.HitActor (Collision|BreakHitResult _outhit))) ; Voir si le laser touche le joueur
    (Components|Timeline|SetPlayRate (Variables|Default|GetTimeline_2) 0.2)
    (bind _opacitymaskvisibility (Timeline|Timeline_2 Play)
      (:Update
        (Rendering|Material|SetScalarParameterValue (Variables|/Game/ThirdPerson/Blueprints/BP_ThirdPersonCharacter.BP_ThirdPersonCharacter_C|GetMaterialBrulure _as_bp_third_person_character) "Visibility" (Math|Float|Lerp 0.0 2.0 _opacitymaskvisibility) :!class /Script/Engine.MaterialInstanceDynamic)
        ;[0 0.3378 1] Effet lors la mort du personnage
        (Effects|Components|ParticleSystem|SetFloatParameter _lasermort "SpawnParticules" 1.0)
        ;;[1 1 1] Lerp de l'apparition des particules
        (bind _newtrack_0 (Timeline|DisparitionParticule PlayFromStart)
          (:Update
            (Effects|Components|ParticleSystem|SetFloatParameter _lasermort "SpawnRate" (Math|Float|Lerp 5e+03 0.0 _newtrack_0))
            (CallFunction|MortPerso) ; Tue le personnage
          ))))
    (else
      ;[1 1 1] Selon si le laser touche une surface, change la taille du laser proportionnellement selon la location de l'impact
      (if (.bBlockingHit (Collision|BreakHitResult _outhit))
        (Niagara|SetNiagaraVariable(Vector3) _ns_piegelaser "BeamEnd" (Math|Vector|MakeVector 0.0 0.0 (.Distance (Collision|BreakHitResult _outhit))))
        ;[1 1 1] Mettre à la place de l'impact le VFX d'étincelle
        (Components|Activation|Activate _spark_2 false)
        (Niagara|SetNiagaraVariable(Float) _spark_2 "BeamSpawnProb" 1.0)
        (Transformation|SetWorldLocation _spark_2 (.Location (Collision|BreakHitResult _outhit)) false false)
        (else
          (Niagara|SetNiagaraVariable(Vector3) _ns_piegelaser "BeamEnd" (Math|Vector|MakeVector 0.0 0.0 (Variables|Laser|GetPorteeMaximaleLaser)))
          (Components|Activation|Deactivate _spark)
          (Niagara|SetNiagaraVariable(Float) _spark "BeamSpawnProb" 0.0))))))

(event EventBeginPlay
  (Utilities|FlowControl|Sequence
    (:then_0
      ;[0 0 0] Caster les différentes références que le BP aura besoin
      ;;[1 1 1] Caster le Game Mode
      (bind _asbp_nano_game_mode (Utilities|Casting|CastToBP_Nano_GameMode (Game|GetGameMode)))
      (Variables|Reference|SetAs%20BP%20Nano%20Game%20Mode _asbp_nano_game_mode))
    (:then_1
      ;;[1 1 1] Caster le BP_ThirdPerson
      (bind _asbp_third_person_character (Utilities|Casting|CastToBP_ThirdPersonCharacter (Game|GetPlayerCharacter 0)))
      (Variables|Reference|SetAs%20BP%20Third%20Person%20Character _asbp_third_person_character))
    (:then_2
      ;[1 0 0.5565] Set les différents éléments au lancement du jeu
      ;;[1 1 1] Attacher le VFX du laser au Mesh
      (Transformation|AttachComponentToComponent (Variables|Default|GetNS_PiegeLaser) (Variables|Default|GetSphere) "None" "KeepRelative" "KeepWorld" "KeepWorld" true)
      ;;[1 1 1] Calcul pour un déplacement conforme selon la distance entre les deux points
      (Components|Timeline|SetPlayRate (Variables|Default|GetTimeline_0) (* (/ 1.0 (.z (Transformation|GetWorldScale (Variables|Default|GetTrail)))) (Variables|Laser|GetVitesseDeplacement)))
      ;;[1 1 1] Mode de déplacement selon si le piège a un mouvement inversé ou pas
      (if (Variables|ModeLaser|GetIsReversed?)
        (CallFunction|Inverse)
        (else
          (CallFunction|AnimationNormal))))))

(fn ConstructionScript
  (bind _sphere (Variables|Default|GetSphere))
  (bind _start (Variables|Default|GetStart))
  (bind _end (Variables|Default|GetEnd))
  (bind _trail (Variables|Default|GetTrail))
  (bind _returnvalue (Transformation|GetWorldLocation _start))
  (bind _returnvalue_2 (Transformation|GetWorldLocation _end))
  (bind _returnvalue_3 (Transformation|GetWorldScale _trail))
  (Utilities|FlowControl|Sequence
    (:then_0
      ;[1 1 1] Changer la taille en Z du trail pour changer en temps réel la distance parcourue par le laser
      (Transformation|SetWorldScale3D _trail (Math|Vector|MakeVector (.x _returnvalue_3) (.y _returnvalue_3) (/ (Variables|Laser|GetDistanceParcourue) 1e+02)))
      ;[1 1 1] Changer la position relatif du point End selon la taille en Z du Trail
      (Transformation|SetRelativeLocation (Variables|Default|GetEnd) (Math|Vector|MakeVector (Variables|Laser|GetDistanceParcourue) 0.0 0.0) false false))
    (:then_1
      (if (Variables|ModeLaser|GetIsReversed?)
        ;[1 1 1] Si inversé, déplace le VFX au point End et fait un mouvement inversé du timeline
        (Transformation|SetWorldLocation _sphere (Math|Vector|MakeVector (.x _returnvalue_2) (.y _returnvalue_2) (+ (Variables|Mesh|GetOffsetMesh) (.z _returnvalue_2))) false false)
        (else
          ;[1 1 1] Si pas inversé, déplace le VFX au point 0 et fait un mouvement pas inversé du timeline
          (Transformation|SetWorldLocation _sphere (Math|Vector|MakeVector (.x _returnvalue) (.y _returnvalue) (+ (.z _returnvalue) (Variables|Mesh|GetOffsetMesh))) false false))))))