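; Fire trap that cycles between flames, pause and smoke warning, killing the player on hitbox overlap with a burn effect.
; Delayed events chain the phases, toggling particles, sound and pipe emissive, with smoke and glow ramping up before each burst.
; A timeline grows the hitbox with the flames and reverses when they stop.
; Per-instance variables set timings, flame height and starting state, with the construction script previewing fire or smoke.
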(event OnComponentBeginOverlap(Hitbox)
  (params (OverlappedComponent :type Primitive%20Component%20Object%20Reference) (OtherActor :type Actor%20Object%20Reference) (OtherComp :type Primitive%20Component%20Object%20Reference) (OtherBodyIndex :type Integer) (bFromSweep :type Boolean) (SweepResult :type Hit%20Result%20Structure%20%28by%20ref%29))
  ;[1 1 1] Mort du personnage lorsqu'il touche les flammes
  (if (== OtherActor (Variables|Reference|GetAs%20BP%20Third%20Person%20Character))
    (Utilities|FlowControl|Sequence
      (:then_0
        (Effects|Components|ParticleSystem|SetFloatParameter (Variables|/Game/ThirdPerson/Blueprints/BP_ThirdPersonCharacter.BP_ThirdPersonCharacter_C|GetFeuMort (Variables|Reference|GetAs%20BP%20Third%20Person%20Character)) "Spawn" 1.0)
        (Utilities|FlowControl|Delay 0.1)
        (Default|Destroy (Variables|Reference|GetAs%20BP%20Third%20Person%20Character) (Variables|Default|GetStringNameDeath)))
      (:then_1
        (bind _newtrack_0 (Timeline|Timeline_0 Play)
          (:Update
            (Rendering|Material|SetScalarParameterValue (Variables|/Game/ThirdPerson/Blueprints/BP_ThirdPersonCharacter.BP_ThirdPersonCharacter_C|GetMaterialBrulure (Variables|Reference|GetAs%20BP%20Third%20Person%20Character)) "IntensityBrulure" (Math|Float|Lerp (Variables|/Game/ThirdPerson/Blueprints/BP_ThirdPersonCharacter.BP_ThirdPersonCharacter_C|GetMaskBrulure (Variables|Reference|GetAs%20BP%20Third%20Person%20Character)) 2.0 _newtrack_0) :!class /Script/Engine.MaterialInstanceDynamic)))))))

(event Custom|ApparitionFlamme
  (bind _feu (Variables|Default|GetFeu))
  (bind _fumee (Variables|Default|GetFumee))
  (Components|Activation|Activate (Variables|Default|GetSonPiegeFeu) false)
  (Audio|Components|Audio|Play (Variables|Default|GetSonPiegeFeu) 0.0)
  (Components|Activation|Deactivate _fumee)
  (Effects|Components|ParticleSystem|SetFloatParameter _fumee "SpawnProb" 0.0)
  (Rendering|Material|SetScalarParameterValue (Variables|Default|GetDynamicMaterialInstanceReference) "Emmisive" 5.0 :!class /Script/Engine.MaterialInstanceDynamic)
  (Utilities|FlowControl|Sequence
    (:then_0
      (Components|Activation|Activate _feu false)
      (Effects|Components|ParticleSystem|SetFloatParameter _feu "SpawnProb" 1.0)
      (Utilities|FlowControl|Delay (Variables|TempsActif|GetTimerActif))
      (CallFunction|DisparitionFlamme))
    (:then_1
      ;[1 1 1] Code pour l'apparition des flammes et changement de forme de la collision pour le feu
      ;;[1 1 1] Change le Play Rate (1.0) avec le temps maximal du mode activé
      (Components|Timeline|SetPlayRate (Variables|Default|GetLongueurTimeline) (/ 1.0 (- (Variables|TempsActif|GetTimerActif) 0.5)))
      ;;[1 1 1] Changer en temps réel la taille de la collision pour augmenter la précision
      (bind _newtrack_0 (Timeline|LongueurTimeline Play)
        (:Update
          (Transformation|SetRelativeScale3D (Variables|Default|GetHitbox) (Math|Vector|MakeVector 1.0 1.0 (Math|Float|Lerp 0.0 (- (/ (Variables|Feu|GetUpdateVelocityMaxFeu) 25.0) 5.0) _newtrack_0))))))))

(event Custom|DisparitionFlamme
  (bind _feu (Variables|Default|GetFeu))
  ;[1 1 1] Quand les flammes disparaissent
  (Components|Activation|Deactivate (Variables|Default|GetSonPiegeFeu))
  (Components|Activation|Activate (Variables|Default|GetSonPiegeFeuFin) false)
  (Components|Activation|Deactivate _feu)
  (Effects|Components|ParticleSystem|SetFloatParameter _feu "SpawnProb" 0.0)
  (Rendering|Material|SetScalarParameterValue (Variables|Default|GetDynamicMaterialInstanceReference) "Emmisive" 0.0 :!class /Script/Engine.MaterialInstanceDynamic)
  (Utilities|FlowControl|Sequence
    (:then_0
      ;;[1 1 1] Fonction pour inverser le Timeline
      (CallFunction|ReverseCollision))
    (:then_1
      ;;[1 1 1] Éteindre les flammes
      (Utilities|FlowControl|Delay (- (Variables|TempsPause|GetTempsPause) 1.0))
      (CallFunction|ApparitionFumee))))

(event Custom|ReverseCollision
  ;[1 1 1] Code pour l'apparition des flammes et changement de forme de la collision pour le feu
  ;;[1 1 1] Inverser la Timeline lorsque le feu est éteint
  (Components|Timeline|SetPlayRate (Variables|Default|GetLongueurTimeline) 0.7)
  ;;[1 1 1] Changer en temps réel la taille de la collision pour augmenter la précision
  (bind _newtrack_0 (Timeline|LongueurTimeline Reverse)
    (:Update
      (Transformation|SetRelativeScale3D (Variables|Default|GetHitbox) (Math|Vector|MakeVector 1.0 1.0 (Math|Float|Lerp 0.0 (- (/ (Variables|Feu|GetUpdateVelocityMaxFeu) 25.0) 5.0) _newtrack_0))))))

(event Custom|Apparition%20Fumee
  (bind _fumee (Variables|Default|GetFumee))
  (bind _fumee_2 (Variables|Default|GetFumee))
  (Components|Activation|Activate _fumee_2 false)
  (Effects|Components|ParticleSystem|SetFloatParameter _fumee_2 "SpawnProb" 1.0)
  (bind (_direction _newtrack_0 _newtrack_1) (Timeline|Opacity%20Lerp PlayFromStart)
    (:Update
      (Effects|Components|ParticleSystem|SetFloatParameter (Variables|Default|GetFumee) "VelociteFumeeMax" (Math|Float|Lerp 0.0 (Variables|Fumee|GetVelociteAnticipitationMax) _newtrack_0))
      (Rendering|Material|SetScalarParameterValue (Variables|Default|GetDynamicMaterialInstanceReference) "Emmisive" (Math|Float|Lerp 0.0 5.0 _newtrack_1) :!class /Script/Engine.MaterialInstanceDynamic))
    (:Finished
      (Components|Activation|Deactivate _fumee)
      (Effects|Components|ParticleSystem|SetFloatParameter _fumee "SpawnProb" 0.0)
      (Utilities|FlowControl|Delay 0.5)
      (CallFunction|ApparitionFlamme))))

(event EventBeginPlay
  (bind _opacity_lerp (Variables|Default|GetOpacity%20Lerp))
  (Utilities|FlowControl|Sequence
    (:then_0
      ;[1 1 1] Caster la référence du joueur
      (bind _asbp_third_person_character (Utilities|Casting|CastToBP_ThirdPersonCharacter (Game|GetPlayerCharacter 0)))
      (Variables|Reference|SetAs%20BP%20Third%20Person%20Character _asbp_third_person_character))
    (:then_1
      ;[1 1 1] Set la vitesse de la timeline de la fumée selon la variable "Pause"
      (Components|Timeline|SetPlayRate _opacity_lerp (/ (- (Components|Animation|GetPlayRate _opacity_lerp) 0.1) (Variables|TempsPause|GetTempsPause))))
    (:then_2
      ;[1 1 1] Créer le matériel qui changera selon le mode actuel
      (bind _returnvalue (Rendering|Material|CreateDynamicMaterialInstance (Variables|Default|GetTuyau) 1 "/Game/Assets/FireTrap/M_Fire_Trap_Emissive.M_Fire_Trap_Emissive" "None" :!class /Script/Engine.PrimitiveComponent))
      (Variables|Default|SetDynamicMaterialInstanceReference _returnvalue))
    (:then_3
      ;[1 1 1] Selon le résultat de la variable, choisir si le piège commence activé ou désactivé dans la scène
      (if (Variables|TempsPause|GetIsPaused?)
        (CallFunction|DisparitionFlamme)
        (else
          (CallFunction|ApparitionFlamme))))))

(fn ConstructionScript
  (bind _feu (Variables|Default|GetFeu))
  (Utilities|FlowControl|Sequence
    (:then_0
      ;[1 1 1] Indiquer dans l'inspecteur la hauteur des flammes
      (Effects|Components|ParticleSystem|SetFloatParameter _feu "FeuVelociteMix" (Variables|Feu|GetUpdateVelocityMinFeu))
      (Effects|Components|ParticleSystem|SetFloatParameter _feu "FeuVelociteMax" (Variables|Feu|GetUpdateVelocityMaxFeu)))
    (:then_1
      (Variables|Default|SetSpawnFeu (/ (Variables|Feu|GetUpdateVelocityMaxFeu) 1e+01))
      (if (Variables|TempsPause|GetIsPaused?)
        ;[1 1 1] Activer la fumee
        (Effects|Components|ParticleSystem|SetFloatParameter (Variables|Default|GetFumee) "SpawnProb" 1.0)
        (Effects|Components|ParticleSystem|SetFloatParameter (Variables|Default|GetFeu) "SpawnProb" 0.0)
        (else
          ;[1 1 1] Activer le feu
          (Effects|Components|ParticleSystem|SetFloatParameter (Variables|Default|GetFeu) "SpawnFeu" (Variables|Default|GetSpawnFeu))
          (Effects|Components|ParticleSystem|SetFloatParameter (Variables|Default|GetFeu) "SpawnProb" 1.0)
          (Effects|Components|ParticleSystem|SetFloatParameter (Variables|Default|GetFumee) "SpawnProb" 0.0))))))

(fn ActiverPiege)

(fn DésactiverPiege)

(fn CalculTempsTimer
  (params (TempsMaximum :type Float%20%28double-precision%29))
  ;[1 1 1] À chaque calcul du timer, ajouter du temps
  (bind _output_get (Variables|Timer|SetMomentTimer (+ (Variables|Timer|GetTick) (Variables|Timer|GetMomentTimer))))
  ;[1 1 1] Si même temps ou plus grand que le temps maximum, change d'étât
  (return (>= _output_get TempsMaximum)))