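; Trigger that ends the tutorial level and sends the player to Main_Level.
; On first player overlap with its collision, it disables shooting, hides the HUD and shows a loading widget.
; Tick polls that widget until it finishes, then once deletes any existing spawn save to avoid bugs and opens the main level after a short delay.
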(event OnComponentBeginOverlap(Collision)
  (params (OverlappedComponent :type Primitive%20Component%20Object%20Reference) (OtherActor :type Actor%20Object%20Reference) (OtherComp :type Primitive%20Component%20Object%20Reference) (OtherBodyIndex :type Integer) (bFromSweep :type Boolean) (SweepResult :type Hit%20Result%20Structure%20%28by%20ref%29))
  ;[1 1 1] Si le joueur overlap la collision
  (if (== OtherActor (Variables|Reference|GetAs%20BP%20Third%20Person%20Character))
    (Utilities|FlowControl|DoOnce false
      (:Completed
        (Default|DesactivationTir (stale EventBeginPlay _output_get))
        (Default|DisparitionHUD (stale EventBeginPlay _output_get_2))
        ;[1 1 1] Message au joueur en disant qu'il changera de niveau
        (bind _returnvalue (UserInterface|CreateWidget "/Game/Blueprint/HUD/HUD_Gameplay/WidgetChargement.WidgetChargement_C"))
        (bind _output_get (Variables|Default|SetNewVar_0 _returnvalue))
        (UserInterface|Viewport|AddtoViewport _returnvalue 0)))))

(event EventBeginPlay
  ;[1 0 0.9914] Begin Play
  ;;[1 1 1] Caster une référence du joueur
  (bind _asbp_third_person_character (Utilities|Casting|CastToBP_ThirdPersonCharacter (Game|GetPlayerCharacter 0)))
  (bind _output_get (Variables|Reference|SetAs%20BP%20Third%20Person%20Character _asbp_third_person_character))
  ;;[1 1 1] Avoir une référence du HUD du joueur
  (bind _ashud_2d (Utilities|Casting|CastToHUD_2D (HUD|GetHUD (Game|GetPlayerController 0))))
  (bind _output_get_2 (Variables|Reference|SetAs%20HUD%202D _ashud_2d)))

(event EventTick
  (params (DeltaSeconds :type Float%20%28single-precision%29))
  (Utilities|IsValid (stale OnComponentBeginOverlap(Collision) _output_get)
    (:Is%20Valid
      (if (Variables|/Game/Blueprint/HUD/HUD_Gameplay/WidgetChargement.WidgetChargement_C|GetIsFinished? (stale OnComponentBeginOverlap(Collision) _output_get))
        (Utilities|FlowControl|DoOnce false
          (:Completed
            ;[1 1 1] Si une sauvegarde existe, l'effacer pour empêcher des bugs possibles
            (bind _returnvalue (SaveGame|DoesSaveGameExist "SauvegardeApparition"))
            (if _returnvalue
              (SaveGame|DeleteGameinSlot "SauvegardeApparition"))
            (Utilities|FlowControl|Delay 0.5)
            (Game|OpenLevel(byName) "Main_Level")))))))

(fn ConstructionScript)