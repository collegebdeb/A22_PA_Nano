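; Test Blueprint for a fire trap that cycles its Fumee smoke VFX on and off, starting shortly after BeginPlay.
; The OpacityLerp timeline, with play rate divided by TempsActivee, ramps the VelociteFumeeMax effect parameter from zero to its maximum, printing each value.
; When it finishes, DisparitionFumee deactivates and zeroes the smoke, waits TempsPause, then loops through Recommencer.
; A separate Restart event and unreached timer logic sit outside this loop.
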(event Custom|ApparitionFumee
  ;[1 1 1] Réactiver le state du VFX
  (Components|Activation|Activate (Variables|Default|GetFumee) false)
  ;[1 1 1] Faire un Lerp selon une timeline pour la velocity de la fumée
  (bind _newtrack_0 (Timeline|OpacityLerp PlayFromStart)
    (:Update
      (Development|PrintString (Utilities|String|ToString(Float) (Math|Float|Lerp 0.0 (Variables|Default|GetVelociteFumeeMax) _newtrack_0)))
      (Effects|Components|ParticleSystem|SetFloatParameter (Variables|Default|GetFumee) "VelociteFumeeMax" (Math|Float|Lerp 0.0 (Variables|Default|GetVelociteFumeeMax) _newtrack_0)))
    (:Finished
      (CallFunction|DisparitionFumee))))

(event Custom|DisparitionFumee
  ;[1 1 1] Faire disparaître la fumée selon un temps imposé. Quand ce temps est finalisé, il se remet en marche
  (Components|Activation|Deactivate (Variables|Default|GetFumee))
  (Effects|Components|ParticleSystem|SetFloatParameter (Variables|Default|GetFumee) "VelociteFumeeMax" 0.0)
  (Utilities|FlowControl|Delay (Variables|Default|GetTempsPause))
  (CallFunction|Recommencer))

(event Custom|Recommencer
  ;[1 1 1] Boucler l'action après la pause
  (CallFunction|ApparitionFumee))

(event Custom|Restart
  (Utilities|FlowControl|DoOnce false ; enters at Reset
    (:Completed
      (Components|Activation|Activate (Variables|Default|GetFumee) false))))

(event EventBeginPlay
  (bind _opacitylerp (Variables|Default|GetOpacityLerp))
  ;[1 1 1] Désactiver le VFX lors du lancement du jeu
  (Components|Activation|Deactivate (Variables|Default|GetFumee))
  (Utilities|FlowControl|Delay 2.0)
  ;[1 1 1] Création du Play Rate conforme selon le temps que l'anticipation sera activée
  (Components|Timeline|SetPlayRate _opacitylerp (/ (Components|Animation|GetPlayRate _opacitylerp) (Variables|Default|GetTempsActivee)))
  (CallFunction|ApparitionFumee))

(fn ConstructionScript)