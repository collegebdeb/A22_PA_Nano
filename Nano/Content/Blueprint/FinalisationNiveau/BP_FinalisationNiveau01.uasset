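; Level-end trigger for level 01 that plays the closing cinematic and returns the player to the main menu.
; When the third-person character overlaps its box with the AllTrue flag set, it hides the HUD and plays the Cinematic_Fin level sequence.
; A looping timer polls the sequence player until playback stops, then clears itself and opens Main_Menu after a short delay.
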(event OnComponentBeginOverlap(Box)
  (params (OverlappedComponent :type Primitive%20Component%20Object%20Reference) (OtherActor :type Actor%20Object%20Reference) (OtherComp :type Primitive%20Component%20Object%20Reference) (OtherBodyIndex :type Integer) (bFromSweep :type Boolean) (SweepResult :type Hit%20Result%20Structure%20%28by%20ref%29))
  (bind _asbp_third_person_character (Utilities|Casting|CastToBP_ThirdPersonCharacter OtherActor))
  (bind _output_get (Variables|Default|SetAs%20BP%20Third%20Person%20Character _asbp_third_person_character))
  (bind _output_get_2 (Variables|Default|SetAs%20HUD%202D (Variables|/Game/ThirdPerson/Blueprints/BP_ThirdPersonCharacter.BP_ThirdPersonCharacter_C|GetHUD _output_get)))
  (if (Variables|/Game/ThirdPerson/Blueprints/BP_ThirdPersonCharacter.BP_ThirdPersonCharacter_C|GetAllTrue _output_get)
    (Default|DisparitionHUD _output_get_2)
    (bind _returnvalue (Sequencer|Player|CreateLevelSequencePlayer "/Game/Cinematic/Cinematic_Fin/Cinematic_Fin.Cinematic_Fin"))
    (Sequencer|Player|Play _returnvalue :!class /Script/MovieScene.MovieSceneSequencePlayer)
    (Utilities|FlowControl|Delay 0.1)
    (bind _returnvalue_2 (Utilities|Time|SetTimerbyEvent (delegate Custom|VoirSiFinit) 0.1 true))))

(event Custom|VoirSiFinit
  (if (not (Audio|Components|Audio|IsPlaying (stale OnComponentBeginOverlap(Box) _returnvalue)))
    (Utilities|Time|ClearandInvalidateTimerbyHandle (stale OnComponentBeginOverlap(Box) _returnvalue_2))
    (Utilities|FlowControl|Delay 1.0)
    (Game|OpenLevel(byName) "Main_Menu")))

(fn ConstructionScript)