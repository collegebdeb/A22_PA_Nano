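; BP_CollisionFinalisationNiveau is a level-completion trigger volume that loads Main_Level when the player character enters it.
; BeginPlay caches the third-person character and the 2D HUD.
; On overlap by that character, a timeline fades the HUD's UI widget render opacity from 0 to 1, then opens the level on finish.
; The construction script sets the collision's scale from an exposed RelativeScale variable.
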(event OnComponentBeginOverlap(Collision)
  (params (OverlappedComponent :type Primitive%20Component%20Object%20Reference) (OtherActor :type Actor%20Object%20Reference) (OtherComp :type Primitive%20Component%20Object%20Reference) (OtherBodyIndex :type Integer) (bFromSweep :type Boolean) (SweepResult :type Hit%20Result%20Structure%20%28by%20ref%29))
  (if (== OtherActor (Variables|Default|GetAs%20BP%20Third%20Person%20Character))
    (bind _newtrack_0 (Timeline|Timeline_0 Play)
      (:Update
        (Widget|SetRenderOpacity (Variables|/Game/Blueprint/HUD/HUD_2D.HUD_2D_C|GetUI_Reference (Variables|Default|GetAs%20HUD%202D)) (Math|Float|Lerp 0.0 1.0 _newtrack_0)))
      (:Finished
        (Game|OpenLevel(byName) "Main_Level")))))

(event EventBeginPlay
  (bind _asbp_third_person_character (Utilities|Casting|CastToBP_ThirdPersonCharacter (Game|GetPlayerCharacter 0)))
  (Variables|Default|SetAs%20BP%20Third%20Person%20Character _asbp_third_person_character)
  (bind _ashud_2d (Utilities|Casting|CastToHUD_2D (HUD|GetHUD (Game|GetPlayerController 0))))
  (Variables|Default|SetAs%20HUD%202D _ashud_2d))

(fn ConstructionScript
  (Transformation|SetRelativeScale3D (Variables|Default|GetCollision) (Variables|Default|GetRelativeScale)))