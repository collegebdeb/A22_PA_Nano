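; BP_PetiteAsteroide is a small asteroid actor, filed among the game's traps, that spins continuously and can explode.
; A looping 60 Hz timer, rather than Tick, adds RotationX to the mesh's relative roll and RotationZ to its yaw, with pitch held at zero.
; A Destruction event spawns an explosion emitter at the asteroid and destroys the actor.
; BeginPlay also caches the player character, though these graphs never use it.
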(event Custom|RotationAsteroide
  (bind _petiteasteroide (Variables|Default|GetPetiteAsteroide))
  (bind _relativerotation (Variables|/Script/Engine.SceneComponent|GetRelativeRotation _petiteasteroide))
  (Utilities|IsValid _petiteasteroide
    (:Is%20Valid
      (Transformation|SetRelativeRotation _petiteasteroide (Math|Rotator|MakeRotator (+ (Variables|Default|GetRotationX) (.roll _relativerotation)) 0.0 (+ (Variables|Default|GetRotationZ) (.yaw _relativerotation))) false false))))

(event EventBeginPlay
  (Utilities|FlowControl|Sequence
    (:then_0
      (Utilities|Time|SetTimerbyEvent (delegate Custom|RotationAsteroide) (/ 1.0 6e+01) true))
    (:then_1
      (bind _asbp_third_person_character (Utilities|Casting|CastToBP_ThirdPersonCharacter (Game|GetPlayerCharacter 0)))
      (Variables|Default|SetAs%20BP%20Third%20Person%20Character _asbp_third_person_character))))

(event EventDestruction
  (Effects|SpawnEmitteratLocation "/Game/VFX/Mine_Explosion/P_Explosion.P_Explosion" (Transformation|GetWorldLocation (Variables|Default|GetPetiteAsteroide)))
  (Actor|DestroyActor))

(fn ConstructionScript)