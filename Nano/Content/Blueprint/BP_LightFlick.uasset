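; Light flicker Blueprint that animates a point light's intensity between a base and a final value.
; BeginPlay sets the base intensity, then IsOn selects TurnOn or TurnOff, which play or reverse a timeline-driven Lerp after a TempsMode delay.
; Timeline completion branches on IsOn again, but every event clears that flag, so it normally re-enters TurnOn.
; BeginOff reverses from the end and has no caller here.
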(event Custom|TurnOn
  (Variables|Default|SetIsOn? false)
  (Utilities|FlowControl|Delay (Variables|Default|GetTempsMode))
  (bind _track_lightflick (Timeline|Timeline_0 Play)
    (:Update
      (Rendering|Components|Light|SetIntensity (Variables|Default|GetPointLight) (Math|Float|Lerp (Variables|Default|GetIntensityBase) (Variables|Default|GetIntensityFinit) _track_lightflick)))
    (:Finished
      (if (Variables|Default|GetIsOn?)
        (Variables|Default|SetIsOn? false)
        (CallFunction|TurnOff)
        (else
          (Variables|Default|SetIsOn? false)
          (CallFunction|Turnon))))))

(event Custom|TurnOff
  (Variables|Default|SetIsOn? false)
  (Utilities|FlowControl|Delay (Variables|Default|GetTempsMode))
  (bind _track_lightflick (Timeline|Timeline_0 Reverse)
    (:Update
      (Rendering|Components|Light|SetIntensity (Variables|Default|GetPointLight) (Math|Float|Lerp (Variables|Default|GetIntensityBase) (Variables|Default|GetIntensityFinit) _track_lightflick)))
    (:Finished
      (if (Variables|Default|GetIsOn?)
        (Variables|Default|SetIsOn? false)
        (CallFunction|TurnOff)
        (else
          (Variables|Default|SetIsOn? false)
          (CallFunction|Turnon))))))

(event Custom|BeginOff
  (Variables|Default|SetIsOn? false)
  (Utilities|FlowControl|Delay (Variables|Default|GetTempsMode))
  (bind _track_lightflick (Timeline|Timeline_0 ReverseFromEnd)
    (:Update
      (Rendering|Components|Light|SetIntensity (Variables|Default|GetPointLight) (Math|Float|Lerp (Variables|Default|GetIntensityBase) (Variables|Default|GetIntensityFinit) _track_lightflick)))
    (:Finished
      (if (Variables|Default|GetIsOn?)
        (Variables|Default|SetIsOn? false)
        (CallFunction|TurnOff)
        (else
          (Variables|Default|SetIsOn? false)
          (CallFunction|Turnon))))))

(event EventBeginPlay
  (Rendering|Components|Light|SetIntensity (Variables|Default|GetPointLight) (Variables|Default|GetIntensityBase))
  (if (Variables|Default|GetIsOn?)
    (CallFunction|Turnon)
    (else
      (CallFunction|TurnOff))))

(fn ConstructionScript)