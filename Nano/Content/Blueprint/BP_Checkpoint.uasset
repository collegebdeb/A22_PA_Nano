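; Checkpoint airlock that refills the player's energy and saves its own transform as the respawn point, once, through BP_Nano_GameMode.
; Overlap volumes drive two timelines that slide the left and right doors along Z.
; The entry door opens on approach and reverses once the player is inside; its Finished pin then opens the exit door if InCheckpoint is set.
; Leaving clears that flag and closes the exit door.
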(event OnComponentBeginOverlap(CollisionOuvrirCheckpoint)
  (params (OverlappedComponent :type Primitive%20Component%20Object%20Reference) (OtherActor :type Actor%20Object%20Reference) (OtherComp :type Primitive%20Component%20Object%20Reference) (OtherBodyIndex :type Integer) (bFromSweep :type Boolean) (SweepResult :type Hit%20Result%20Structure%20%28by%20ref%29))
  (bind _relativepositionportegauche (Variables|Animation|GetRelativePositionPorteGauche))
  (bind _relativepositionportedroite (Variables|Animation|GetRelativePositionPorteDroite))
  (bind _as_bp_third_person_character (Variables|Reference|GetAs%20BP%20Third%20Person%20Character))
  (if (== OtherActor (Variables|Reference|GetAs%20BP%20Third%20Person%20Character))
    ;[1 1 1] Timeline (Opacity)
    (bind _opacity_animation (Timeline|AnimationTransform Play)
      (:Update
        ;[1 1 1] Créer l'animation de la porte gauche (ouverture)
        (Transformation|SetRelativeLocation (Variables|Default|GetPorteGauche) (Math|Vector|MakeVector (.x _relativepositionportegauche) (.y _relativepositionportegauche) (+ (.z _relativepositionportegauche) (Math|Float|Lerp 0.0 (Variables|Animation|GetDeplacementPorte) _opacity_animation))) false false))
      (:Finished
        (Utilities|IsValid _as_bp_third_person_character
          (:Is%20Valid
            ;[1 1 1] Si le joueur est dans le checkpoint, joue l'animation qui ouvre la porte droite
            (if (Variables|/Game/ThirdPerson/Blueprints/BP_ThirdPersonCharacter.BP_ThirdPersonCharacter_C|GetIn%20Checkpoint? _as_bp_third_person_character)
              (Utilities|FlowControl|Delay 0.5)
              (bind _opacity_animation_2 (Timeline|Timeline_0 Play)
                (:Update
                  (Transformation|SetRelativeLocation (Variables|Default|GetPorteDroite) (Math|Vector|MakeVector (.x _relativepositionportedroite) (.y _relativepositionportedroite) (+ (.z _relativepositionportedroite) (Math|Float|Lerp 0.0 (Variables|Animation|GetDeplacementPorte) _opacity_animation_2))) false false))))))))))

(event OnComponentBeginOverlap(Box)
  (params (OverlappedComponent :type Primitive%20Component%20Object%20Reference) (OtherActor :type Actor%20Object%20Reference) (OtherComp :type Primitive%20Component%20Object%20Reference) (OtherBodyIndex :type Integer) (bFromSweep :type Boolean) (SweepResult :type Hit%20Result%20Structure%20%28by%20ref%29))
  (bind _defaultsceneroot (Variables|Default|GetDefaultSceneRoot))
  (bind _as_bp_third_person_character (Variables|Reference|GetAs%20BP%20Third%20Person%20Character))
  (if (== OtherActor _as_bp_third_person_character)
    (Variables|/Game/ThirdPerson/Blueprints/BP_ThirdPersonCharacter.BP_ThirdPersonCharacter_C|SetEnergieActuelle _as_bp_third_person_character (Variables|/Game/ThirdPerson/Blueprints/BP_ThirdPersonCharacter.BP_ThirdPersonCharacter_C|GetEnergieLimite _as_bp_third_person_character))
    (Variables|/Game/ThirdPerson/Blueprints/BP_ThirdPersonCharacter.BP_ThirdPersonCharacter_C|SetIn%20Checkpoint? _as_bp_third_person_character true)
    (Utilities|FlowControl|DoOnce false
      (:Completed
        (Default|UpdateApparitionSave (Variables|Reference|GetAs%20BP%20Nano%20Game%20Mode) (Math|Transform|MakeTransform (Transformation|GetWorldLocation _defaultsceneroot) (Transformation|GetWorldRotation _defaultsceneroot)))))))

(event OnComponentBeginOverlap(Collision)
  (params (OverlappedComponent :type Primitive%20Component%20Object%20Reference) (OtherActor :type Actor%20Object%20Reference) (OtherComp :type Primitive%20Component%20Object%20Reference) (OtherBodyIndex :type Integer) (bFromSweep :type Boolean) (SweepResult :type Hit%20Result%20Structure%20%28by%20ref%29))
  ;[1 1 1] Lorsque le joueur entre dans la zone de sauvegarde
  (if (== OtherActor (Variables|Reference|GetAs%20BP%20Third%20Person%20Character))
    (CallFunction|FermeturePorte)))

(event OnComponentEndOverlap(Collision)
  (params (OverlappedComponent :type Primitive%20Component%20Object%20Reference) (OtherActor :type Actor%20Object%20Reference) (OtherComp :type Primitive%20Component%20Object%20Reference) (OtherBodyIndex :type Integer))
  ;[1 1 1] Lorsque le joueur quitte la zone, les propulseurs regagnent la possibilité d'épuiser de l'énergie (Inverse l'animation de la porte droite aussi)
  (if (== OtherActor (Variables|Reference|GetAs%20BP%20Third%20Person%20Character))
    (Variables|/Game/ThirdPerson/Blueprints/BP_ThirdPersonCharacter.BP_ThirdPersonCharacter_C|SetIn%20Checkpoint? (Variables|Reference|GetAs%20BP%20Third%20Person%20Character) false)))

(event OnComponentEndOverlap(Box)
  (params (OverlappedComponent :type Primitive%20Component%20Object%20Reference) (OtherActor :type Actor%20Object%20Reference) (OtherComp :type Primitive%20Component%20Object%20Reference) (OtherBodyIndex :type Integer))
  (bind _as_bp_third_person_character (Variables|Reference|GetAs%20BP%20Third%20Person%20Character))
  (bind _relativepositionportedroite (Variables|Animation|GetRelativePositionPorteDroite))
  (if (and (== OtherActor _as_bp_third_person_character) (not (Variables|/Game/ThirdPerson/Blueprints/BP_ThirdPersonCharacter.BP_ThirdPersonCharacter_C|GetIn%20Checkpoint? _as_bp_third_person_character)))
    (Utilities|FlowControl|Delay 0.5)
    ;[1 1 1] Si le joueur est dans le checkpoint, joue l'animation qui ouvre la porte droite
    (bind _opacity_animation (Timeline|Timeline_0 Reverse)
      (:Update
        (Transformation|SetRelativeLocation (Variables|Default|GetPorteDroite) (Math|Vector|MakeVector (.x _relativepositionportedroite) (.y _relativepositionportedroite) (+ (.z _relativepositionportedroite) (Math|Float|Lerp 0.0 (Variables|Animation|GetDeplacementPorte) _opacity_animation))) false false)))))

(event Custom|FermeturePorte
  (bind _relativepositionportegauche (Variables|Animation|GetRelativePositionPorteGauche))
  (bind _relativepositionportedroite (Variables|Animation|GetRelativePositionPorteDroite))
  (bind _as_bp_third_person_character (Variables|Reference|GetAs%20BP%20Third%20Person%20Character))
  (Utilities|FlowControl|Delay 0.5)
  ;[1 1 1] Timeline (Opacity)
  (bind _opacity_animation (Timeline|AnimationTransform Reverse)
    (:Update
      ;[1 1 1] Créer l'animation de la porte gauche (ouverture)
      (Transformation|SetRelativeLocation (Variables|Default|GetPorteGauche) (Math|Vector|MakeVector (.x _relativepositionportegauche) (.y _relativepositionportegauche) (+ (.z _relativepositionportegauche) (Math|Float|Lerp 0.0 (Variables|Animation|GetDeplacementPorte) _opacity_animation))) false false))
    (:Finished
      (Utilities|IsValid _as_bp_third_person_character
        (:Is%20Valid
          ;[1 1 1] Si le joueur est dans le checkpoint, joue l'animation qui ouvre la porte droite
          (if (Variables|/Game/ThirdPerson/Blueprints/BP_ThirdPersonCharacter.BP_ThirdPersonCharacter_C|GetIn%20Checkpoint? _as_bp_third_person_character)
            (Utilities|FlowControl|Delay 0.5)
            (bind _opacity_animation_2 (Timeline|Timeline_0 Play)
              (:Update
                (Transformation|SetRelativeLocation (Variables|Default|GetPorteDroite) (Math|Vector|MakeVector (.x _relativepositionportedroite) (.y _relativepositionportedroite) (+ (.z _relativepositionportedroite) (Math|Float|Lerp 0.0 (Variables|Animation|GetDeplacementPorte) _opacity_animation_2))) false false)))))))))

(event EventBeginPlay
  (Utilities|FlowControl|Sequence
    (:then_0
      ;[1 1 1] Sauvegarder Personnage
      (bind _asbp_third_person_character (Utilities|Casting|CastToBP_ThirdPersonCharacter (Game|GetPlayerCharacter 0)))
      (Variables|Reference|SetAs%20BP%20Third%20Person%20Character _asbp_third_person_character))
    (:then_1
      ;[1 1 1] Sauvegarder Game Mode
      (bind _asbp_nano_game_mode (Utilities|Casting|CastToBP_Nano_GameMode (Game|GetGameMode)))
      (Variables|Reference|SetAs%20BP%20Nano%20Game%20Mode _asbp_nano_game_mode))
    (:then_2
      ;[1 1 1] Avoir la position de la porte gauche
      (Variables|Animation|SetRelativePositionPorteGauche (Variables|/Script/Engine.SceneComponent|GetRelativeLocation (Variables|Default|GetPorteGauche))))
    (:then_3
      ;[1 1 1] Avoir la position de la porte droite
      (Variables|Animation|SetRelativePositionPorteDroite (Variables|/Script/Engine.SceneComponent|GetRelativeLocation (Variables|Default|GetPorteDroite))))))

(fn ConstructionScript)