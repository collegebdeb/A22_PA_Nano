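; BP_PiegeMine is a mine trap that explodes and kills the player on contact.
; On BeginPlay it caches the third-person character, and its Hitbox overlap reacts only to that actor.
; Contact calls DestroyMine, which spawns a scaled explosion emitter, plays a sound and destroys the mine, then calls the character's Destroy.
; A DestructionMeteorite event shares the same explosion logic without affecting the player.
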(event OnComponentBeginOverlap(Hitbox)
  (params (OverlappedComponent :type Primitive%20Component%20Object%20Reference) (OtherActor :type Actor%20Object%20Reference) (OtherComp :type Primitive%20Component%20Object%20Reference) (OtherBodyIndex :type Integer) (bFromSweep :type Boolean) (SweepResult :type Hit%20Result%20Structure%20%28by%20ref%29))
  ;[1 1 1] Lorsque le joueur entre en collision avec la mine
  (if (== OtherActor (Variables|Reference|GetAs%20BP%20Third%20Person%20Character))
    (Utilities|FlowControl|Sequence
      (:then_0
        ;[1 1 1] Destruction Mine
        (CallFunction|DestroyMine))
      (:then_1
        ;[1 1 1] Destruction Joueur
        (Default|Destroy (Variables|Reference|GetAs%20BP%20Third%20Person%20Character))))))

(event Custom|DestroyMine
  ;[1 1 1] Explosion lors de la destruction de la mine
  (Effects|SpawnEmitteratLocation "/Game/VFX/Mine_Explosion/P_Explosion.P_Explosion" (Transformation|GetWorldLocation (Variables|Default|GetCube)) "0, 0, 0" "3.000000,3.000000,3.000000")
  (Audio|PlaySound2D "/Game/Sons/ExplosionMine.ExplosionMine" 1.0 1.0 0.0 0 0)
  (Actor|DestroyActor))

(event EventBeginPlay
  ;[1 1 1] Caster la référence du joueur
  (bind _asbp_third_person_character (Utilities|Casting|CastToBP_ThirdPersonCharacter (Game|GetPlayerCharacter 0)))
  (Variables|Reference|SetAs%20BP%20Third%20Person%20Character _asbp_third_person_character))

(event EventDestructionMeteorite
  ;[1 1 1] Explosion lors de la destruction de la mine
  (Effects|SpawnEmitteratLocation "/Game/VFX/Mine_Explosion/P_Explosion.P_Explosion" (Transformation|GetWorldLocation (Variables|Default|GetCube)) "0, 0, 0" "3.000000,3.000000,3.000000")
  (Audio|PlaySound2D "/Game/Sons/ExplosionMine.ExplosionMine" 1.0 1.0 0.0 0 0)
  (Actor|DestroyActor))

(fn ConstructionScript)