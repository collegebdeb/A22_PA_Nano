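; Meteorite spawner trap that repeatedly launches a small meteorite along a configurable trajectory.
; After a pause, it spawns BP_MeteoritePetite at the Spawner transform and uses MoveComponentTo to slide and rotate its Meteorite component over a set duration.
; When the move completes, it destroys the meteorite and restarts the cycle.
; The construction script sets the Spawner pitch and places the FinTrajectoire end marker from the length setting, also used as the move target.
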(event Custom|DestroyMeteorite
  (CallFunction|Stop)
  (Actor|DestroyActor (Variables|Default|GetNewVar_0))
  (CallFunction|RespawnObject))

(event Custom|RespawnObject
  (bind _dureetransition (Variables|Default|GetDureeTransition))
  (bind _returnvalue (* _dureetransition 2e+01))
  (Utilities|FlowControl|Delay (Variables|Default|GetPauseEntreSpawn))
  (bind _output_get1 (CallFunction|ApparitionMeteorite))
  (bind _output_get (Variables|Default|SetNewVar_0 _output_get1))
  (Utilities|IsValid _output_get
    (:Is%20Valid
      (Components|MoveComponentTo (Variables|/Game/Blueprint/Pièges/BP_MeteoritePetite.BP_MeteoritePetite_C|GetMeteorite _output_get1) (Variables|Default|GetNewVar_1) (Math|Rotator|MakeRotator _returnvalue _returnvalue 0.0) false false (Variables|Default|GetDureeTransition) false)
      (CallFunction|DestroyMeteorite))))

(event Custom|Stop
  (bind _dureetransition (Variables|Default|GetDureeTransition))
  (bind _returnvalue (* _dureetransition 2e+01))
  (Components|MoveComponentTo (Variables|/Game/Blueprint/Pièges/BP_MeteoritePetite.BP_MeteoritePetite_C|GetMeteorite (stale Custom|RespawnObject _output_get1)) (Variables|Default|GetNewVar_1) (Math|Rotator|MakeRotator _returnvalue _returnvalue 0.0) false false (Variables|Default|GetDureeTransition) false) ; enters at Stop
)

(event EventBeginPlay
  (bind _dureetransition (Variables|Default|GetDureeTransition))
  (bind _returnvalue (* _dureetransition 2e+01))
  (Utilities|FlowControl|Delay (Variables|Default|GetPauseEntreSpawn))
  (bind _output_get1 (CallFunction|ApparitionMeteorite))
  (bind _output_get (Variables|Default|SetNewVar_0 _output_get1))
  (Utilities|IsValid _output_get
    (:Is%20Valid
      (Components|MoveComponentTo (Variables|/Game/Blueprint/Pièges/BP_MeteoritePetite.BP_MeteoritePetite_C|GetMeteorite _output_get1) (Variables|Default|GetNewVar_1) (Math|Rotator|MakeRotator _returnvalue _returnvalue 0.0) false false (Variables|Default|GetDureeTransition) false)
      (CallFunction|DestroyMeteorite))))

(fn ConstructionScript
  (bind _spawner (Variables|Default|GetSpawner))
  (bind _spawner_2 (Variables|Default|GetSpawner))
  (bind _relativelocation (Variables|/Script/Engine.SceneComponent|GetRelativeLocation _spawner_2))
  (bind _relativerotation (Variables|/Script/Engine.SceneComponent|GetRelativeRotation _spawner))
  (Utilities|FlowControl|Sequence
    (:then_0
      (Transformation|SetRelativeRotation (Variables|Default|GetSpawner) (Math|Rotator|MakeRotator (.roll _relativerotation) (Variables|Default|GetRotationPositionMeteorite) (.yaw _relativerotation)) false false))
    (:then_1
      (bind _output_get (Variables|Default|SetNewVar_1 (Math|Vector|MakeVector (Variables|Default|GetLongueurTransformation) (.y _relativelocation) (.z _relativelocation))))
      (Transformation|SetRelativeLocation (Variables|Default|GetFinTrajectoire) _output_get false false))))

(fn ApparitionMeteorite
  (bind _returnvalue (Game|SpawnActorfromClass "/Game/Blueprint/Pièges/BP_MeteoritePetite.BP_MeteoritePetite_C" (Transformation|GetWorldTransform (Variables|Default|GetSpawner)) "Undefined" 0 0))
  (bind _output_get (Variables|Default|SetNewVar_0 _returnvalue))
  (return _output_get))