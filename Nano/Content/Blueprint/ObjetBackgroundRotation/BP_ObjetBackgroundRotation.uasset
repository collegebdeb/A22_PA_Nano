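; Background prop Blueprint that displays a configurable mesh spinning at a random rate.
; The construction script applies the Objet mesh to its StaticMesh component.
; On BeginPlay, it sets the RotatingMovement rotation rate once, drawing each axis between zero and its editor-tunable maximum (RandomX, RandomY, RandomZ), so each instance rotates differently.
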(event EventBeginPlay
  ;[1 1 1] Créer un rotator selon des floats modifiable dans l'éditeur
  (Variables|/Script/Engine.RotatingMovementComponent|SetRotationRate (Variables|Default|GetRotatingMovement) (Math|Rotator|MakeRotator (Math|Random|RandomFloatinRange 0.0 (Variables|Rotation|GetRandom_X)) (Math|Random|RandomFloatinRange 0.0 (Variables|Rotation|GetRandom_Y)) (Math|Random|RandomFloatinRange 0.0 (Variables|Rotation|GetRandom_Z)))))

(fn ConstructionScript
  ;[1 1 1] Mettre un StaticMesh au millieu de l'objet
  (Components|StaticMesh|SetStaticMesh (Variables|Default|GetStaticMesh) (Variables|Objet|GetObjet)))