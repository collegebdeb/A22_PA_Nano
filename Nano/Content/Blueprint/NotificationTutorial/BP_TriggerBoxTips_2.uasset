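; Tutorial tip trigger box that shows a notification widget and pauses the game when the player enters it.
; BeginPlay caches the player's BP_ThirdPersonCharacter to filter overlaps, and a DoOnce limits the tip to the first entry.
; That overlap creates the widget, adds it to the viewport, fades it in with the Opacity timeline, then pauses on completion.
; The file has no fade-out, removal or unpause logic.
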(event Collision|EventActorBeginOverlap
  (params (OtherActor :type Actor%20Object%20Reference))
  ;[1 1 1] Événement qui arrive lorsque le joueur entre dans le triggerbox
  ;;[1 1 1] Voir si le joueur overlap le triggerbox
  (if (== OtherActor (Variables|Default|GetAs%20BP%20Third%20Person%20Character))
    (Utilities|FlowControl|DoOnce false
      (:Completed
        ;[1 1 1] Création et affichage initiale du widget lorsque le triggerbox overlap avec le joueur ou celui-ci attends un certain temps
        ;;[1 1 1] Créer le widget, changer le texte à l'intérieur et change le texte existant avec celui modifier dans le triggerbox
        (bind _returnvalue (UserInterface|CreateWidget (Variables|Default|GetClass) (Game|GetPlayerController 0)))
        (Variables|Default|SetWidgetIsExisting? true)
        (bind _output_get (Variables|Default|SetNewVar_0 _returnvalue))
        ;;[1 1 1] Mettre le widget dans le viewport du joueur. Mettre l'opacity à 0
        (UserInterface|Viewport|AddtoViewport _output_get 0)
        (Widget|SetRenderOpacity _output_get 0.0)
        ;[1 1 1] Animation et Lerp de l'opacity du widget pour un fade-in/fade-out
        ;;[1 1 1] Set l'opacity selon si le joueur entre, quitte ou attends pendant un temps dans le triggerbox
        (bind _newtrack_0 (Timeline|Opacity PlayFromStart)
          (:Update
            (Widget|SetRenderOpacity (Variables|Default|GetNewVar_0) (Math|Float|Lerp 0.0 1.0 _newtrack_0)))
          (:Finished
            (Game|SetGamePaused true)))))))

(event EventBeginPlay
  ;[1 1 1] Caster le joueur comme référence de collision possible avec le triggerbox
  (bind _asbp_third_person_character (Utilities|Casting|CastToBP_ThirdPersonCharacter (Game|GetPlayerCharacter 0)))
  (Variables|Default|SetAs%20BP%20Third%20Person%20Character _asbp_third_person_character))

(fn ConstructionScript)