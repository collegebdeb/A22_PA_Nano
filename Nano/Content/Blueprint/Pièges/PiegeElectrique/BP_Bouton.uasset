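; Shootable button that shuts down its linked electric traps once its health is depleted.
; The Destruction event subtracts shot damage; at zero it plays a one-time Zone 1 cinematic and sound, toggling player input off and back on.
; A timeline then fades the emissive on a dynamic material instance created at BeginPlay, and calls ArretPiege on each linked trap when finished.
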(event EventDestruction
  (params (TirDegatParTir :type Integer) (DeltaTime :type Float%20%28double-precision%29))
  ;[1 1 1] Réduction des PVs du bouton
  (bind _output_get (Variables|Default|SetPV (- (Variables|Default|GetPV) (* TirDegatParTir 1))))
  ;[1 1 1] Voir si PV atteint O
  (if (<= _output_get 0)
    (Utilities|FlowControl|DoOnce false
      (:Completed
        ;[1 1 1] Bloque le mouvement du joueur
        (Input|DisableInput (Game|GetPlayerCharacter 0) (Game|GetPlayerController 0))
        ;[1 1 1] Permet de jouer la cinématique
        (bind _returnvalue (Sequencer|Player|CreateLevelSequencePlayer "/Game/Cinematic/Cinematic_Piege/Cinematic_Zone1.Cinematic_Zone1"))
        (bind _output_get_2 (Variables|Default|SetVariableCinematique _returnvalue))
        (Sequencer|Player|Play _output_get_2 :!class /Script/MovieScene.MovieSceneSequencePlayer)
        (Audio|SpawnSound2D "/Game/Sons/PiegeElectrique/BoutonPiege.BoutonPiege" 1.0 1.0 0.0 0)
        ;[1 1 1] Permet le joueur de bouger
        (Utilities|FlowControl|DoOnce false
          (:Completed
            (Input|EnableInput (Game|GetPlayerCharacter 0) (Game|GetPlayerController 0))
            ;[1 1 1] Changement (en temps réel), de l'emissive du bouton
            (bind _newtrack_0 (Timeline|DisparitionBoule Play)
              (:Update
                (Rendering|Material|SetScalarParameterValue (Variables|Default|GetMaterialEmissive) "EmissiveIntensity" (Math|Float|Lerp 0.5 0.0 _newtrack_0) :!class /Script/Engine.MaterialInstanceDynamic))
              (:Finished
                ;[1 1 1] Détruire la référence à chacun des boutons
                (for _array_element (Variables|Default|GetPiegeElectrique)
                  (Default|ArretPiege _array_element))))))))))

(event EventBeginPlay
  ;[1 1 1] Création du matérial dynamique pour l'emissive du bouton
  (bind _returnvalue (Rendering|Material|CreateDynamicMaterialInstance "/Game/Assets/Trap_Button/boton.boton" "None" "None" :!class /Script/Engine.KismetMaterialLibrary))
  (bind _output_get (Variables|Default|SetMaterialEmissive _returnvalue))
  (bind _returnvalue_2 (Rendering|Material|GetScalarParameterValue _output_get "EmissiveIntensity" :!class /Script/Engine.MaterialInstanceDynamic))
  (Variables|Default|SetIntensityBase _returnvalue_2)
  (Rendering|Material|SetMaterial (Variables|Default|GetAccesoire2) 0 _output_get))

(fn ConstructionScript)