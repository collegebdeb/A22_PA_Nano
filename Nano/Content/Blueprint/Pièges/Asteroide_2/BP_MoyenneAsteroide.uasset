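; BP_MoyenneAsteroide is a medium asteroid trap that breaks into two spawned actors when destroyed.
; Its Destruction event plays a scaled-up explosion emitter at the asteroid's location.
; It then spawns two actors there with random pitch in opposite directions, one positive and one negative, so they diverge, and destroys itself.
; BeginPlay and the construction script are empty.
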(event EventBeginPlay)

(event EventDestruction
  (bind _moyenneasteroide (Variables|Default|GetMoyenneAsteroide))
  (bind _returnvalue (Transformation|GetWorldTransform _moyenneasteroide))
  (Effects|SpawnEmitteratLocation "/Game/VFX/Mine_Explosion/P_Explosion.P_Explosion" (Transformation|GetWorldLocation _moyenneasteroide) "0, 0, 0" "2.000000,2.000000,2.000000")
  (Utilities|FlowControl|Sequence
    (:then_0
      (Game|SpawnActorfromClass (Variables|Default|GetClass) (Math|Transform|MakeTransform (.location _returnvalue) (Math|Rotator|MakeRotator 0.0 (Math|Random|RandomFloatinRange 5.0 15.0) 0.0) "1.000000,1.000000,1.000000") "Undefined" 0 0))
    (:then_1
      (Game|SpawnActorfromClass (Variables|Default|GetClass) (Math|Transform|MakeTransform (.location _returnvalue) (Math|Rotator|MakeRotator 0.0 (Math|Random|RandomFloatinRange -5.0 -15.0) 0.0) "1.000000,1.000000,1.000000") "Undefined" 0 0))
    (:then_2
      (Actor|DestroyActor))))

(fn ConstructionScript)