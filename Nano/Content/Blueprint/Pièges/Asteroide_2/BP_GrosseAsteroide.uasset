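; BP_GrosseAsteroide is a large asteroid actor that continuously tumbles in place.
; On BeginPlay, a looping 60 Hz timer adds the RotationX and RotationZ steps to the mesh's relative roll and yaw, holding pitch at zero.
; BeginPlay also caches the player's ThirdPersonCharacter, which this graph does not otherwise use.
; The Destruction and DestructionGrosse events are empty stubs.
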(event Custom|DestructionGrosse)

(event Custom|RotationAsteroide
  (bind _grosseasteroide (Variables|Default|GetGrosseAsteroide))
  (bind _grosseasteroide_2 (Variables|Default|GetGrosseAsteroide))
  (bind _relativerotation (Variables|/Script/Engine.SceneComponent|GetRelativeRotation _grosseasteroide))
  (Utilities|IsValid _grosseasteroide_2
    (:Is%20Valid
      (Transformation|SetRelativeRotation _grosseasteroide_2 (Math|Rotator|MakeRotator (+ (Variables|Rotation|GetRotationX) (.roll _relativerotation)) 0.0 (+ (Variables|Rotation|GetRotationZ) (.yaw _relativerotation))) false false))))

(event EventBeginPlay
  (Utilities|FlowControl|Sequence
    (:then_0
      (Utilities|Time|SetTimerbyEvent (delegate Custom|RotationAsteroide) (/ 1.0 6e+01) true))
    (:then_1
      (bind _asbp_third_person_character (Utilities|Casting|CastToBP_ThirdPersonCharacter (Game|GetPlayerCharacter 0)))
      (Variables|Default|SetAs%20BP%20Third%20Person%20Character _asbp_third_person_character))))

(event EventDestruction)

(fn ConstructionScript)