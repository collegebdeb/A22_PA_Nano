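; Base meteorite trap spawner that launches actors of a configurable class from its sphere along an arrow set in construction.
; While active, it spawns on BeginPlay or via Actif, repeating after a delay unless one-shot.
; Each meteorite gets a runtime ProjectileMovementComponent with a configurable max speed and joins an array.
; A looping timer trims that array over its cap, destroying the oldest valid meteorite with a Niagara explosion.
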(event Custom|SpawnAnother
  (bind _array_spawnactor (Variables|Components|GetArray_SpawnActor))
  ;[1 1 1] Spawn un acteur du type "Météorite"
  (if (Variables|Actif|GetIsActif?)
    (bind _returnvalue (Game|SpawnActorfromClass (Variables|Components|GetTypeClassMeteorite) (Math|Transform|MakeTransform (Transformation|GetWorldLocation (Variables|Default|GetSphere)) (Variables|/Script/Engine.SceneComponent|GetRelativeRotation (Variables|Default|GetArrow)) "1.000000,1.000000,1.000000") "Undefined" 0 0))
    ;[1 1 1] Placer chaque acteur dans un tableau et lui attacher un projectile component
    (bind _output_get (Variables|Components|SetSpawnActor _returnvalue))
    (bind _returnvalue_2 (Utilities|Array|Add _array_spawnactor _output_get))
    (bind _returnvalue_3 (AddComponent|AddProjectileMovementComponent (Utilities|Array|Get(acopy) _array_spawnactor _returnvalue_2)))
    ;[1 1 1] Changer la velocity de l'objet
    (bind _output_get_2 (Variables|Default|SetProjectileComponent _returnvalue_3))
    (Variables|/Script/Engine.ProjectileMovementComponent|SetMaxSpeed _output_get_2 (Variables|Spawn|GetVelocityProjectile))
    (if (not (Variables|Actif|GetOnlyOneTime?))
      ;[1 1 1] Temps entre chaque apparition
      (Utilities|FlowControl|Delay (Variables|Spawn|GetTempsEntreApparition))
      (CallFunction|SpawnAnother))))

(event Custom|VoirSiLimiteAtteint
  (bind _array_spawnactor (Variables|Components|GetArray_SpawnActor))
  (bind _output (Utilities|Array|Get(acopy) _array_spawnactor))
  ;[1 1 1] Voir si la longueur du tableau est plus elevé que la limite possible. Si oui, essaie de voir si l'acteur est valide
  (if (> (Utilities|Array|Length _array_spawnactor) (Variables|Spawn|GetNombreMaximaleSpawnMeteorite))
    ;;[1 1 1] Voir si le premier index du tableau est valide et pas détruit
    (Utilities|IsValid _output
      (:Is%20Valid
        ;[1 1 1] Changer les valeurs du spawn emitter lorsque la météorite est détruite
        (Niagara|SpawnSystematLocation "/Game/VFX/Meteorite_Explosion/Explosion_Meteorite.Explosion_Meteorite" (Transformation|GetWorldLocation (Variables|/Script/Engine.Actor|GetRootComponent _output)) "0, 0, 0" (Variables|VFX|GetScaleEmitter))
        ;[1 1 1] Détruire et l'enlever du tableau
        (Actor|DestroyActor _output)
        (Utilities|Array|RemoveIndex _array_spawnactor)))))

(event Custom|Actif
  (bind _array_spawnactor (Variables|Components|GetArray_SpawnActor))
  ;[1 1 1] Spawn un acteur du type "Météorite"
  (if (Variables|Actif|GetIsActif?)
    (bind _returnvalue (Game|SpawnActorfromClass (Variables|Components|GetTypeClassMeteorite) (Math|Transform|MakeTransform (Transformation|GetWorldLocation (Variables|Default|GetSphere)) (Variables|/Script/Engine.SceneComponent|GetRelativeRotation (Variables|Default|GetArrow)) "1.000000,1.000000,1.000000") "Undefined" 0 0))
    ;[1 1 1] Placer chaque acteur dans un tableau et lui attacher un projectile component
    (bind _output_get (Variables|Components|SetSpawnActor _returnvalue))
    (bind _returnvalue_2 (Utilities|Array|Add _array_spawnactor _output_get))
    (bind _returnvalue_3 (AddComponent|AddProjectileMovementComponent (Utilities|Array|Get(acopy) _array_spawnactor _returnvalue_2)))
    ;[1 1 1] Changer la velocity de l'objet
    (bind _output_get_2 (Variables|Default|SetProjectileComponent _returnvalue_3))
    (Variables|/Script/Engine.ProjectileMovementComponent|SetMaxSpeed _output_get_2 (Variables|Spawn|GetVelocityProjectile))
    (if (not (Variables|Actif|GetOnlyOneTime?))
      ;[1 1 1] Temps entre chaque apparition
      (Utilities|FlowControl|Delay (Variables|Spawn|GetTempsEntreApparition))
      (CallFunction|SpawnAnother))))

(event EventBeginPlay
  (bind _array_spawnactor (Variables|Components|GetArray_SpawnActor))
  ;[1 1 1] Créer un un Update Tick personnalisé pour voir si le spawner a atteint la limite d'objet possible
  (Utilities|Time|SetTimerbyEvent (delegate Custom|VoirSiLimiteAtteint) 0.1 true)
  ;[1 1 1] Spawn un acteur du type "Météorite"
  (if (Variables|Actif|GetIsActif?)
    (bind _returnvalue (Game|SpawnActorfromClass (Variables|Components|GetTypeClassMeteorite) (Math|Transform|MakeTransform (Transformation|GetWorldLocation (Variables|Default|GetSphere)) (Variables|/Script/Engine.SceneComponent|GetRelativeRotation (Variables|Default|GetArrow)) "1.000000,1.000000,1.000000") "Undefined" 0 0))
    ;[1 1 1] Placer chaque acteur dans un tableau et lui attacher un projectile component
    (bind _output_get (Variables|Components|SetSpawnActor _returnvalue))
    (bind _returnvalue_2 (Utilities|Array|Add _array_spawnactor _output_get))
    (bind _returnvalue_3 (AddComponent|AddProjectileMovementComponent (Utilities|Array|Get(acopy) _array_spawnactor _returnvalue_2)))
    ;[1 1 1] Changer la velocity de l'objet
    (bind _output_get_2 (Variables|Default|SetProjectileComponent _returnvalue_3))
    (Variables|/Script/Engine.ProjectileMovementComponent|SetMaxSpeed _output_get_2 (Variables|Spawn|GetVelocityProjectile))
    (if (not (Variables|Actif|GetOnlyOneTime?))
      ;[1 1 1] Temps entre chaque apparition
      (Utilities|FlowControl|Delay (Variables|Spawn|GetTempsEntreApparition))
      (CallFunction|SpawnAnother))))

(fn ConstructionScript
  (Transformation|SetRelativeRotation (Variables|Default|GetArrow) (Variables|Rotation|GetRotationApparitionMeteorite) false false))

(fn ParametreMeteorite
  (params (ProjectileComponent :type Projectile%20Movement%20Component%20Object%20Reference)))