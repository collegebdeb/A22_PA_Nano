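; Parent Blueprint for energy collectibles that the player picks up to refill an energy gauge.
; On BeginPlay it caches the player character and runs a timeline that alternates forward and reverse, lerping the Scene component's relative Z for an up-and-down float.
; When the capsule overlaps that player, it plays a pickup sound, then after a short delay a battery-gain sound, destroys itself and passes ValeurEnergie to RecevoirBonusEnergie.
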(event OnComponentBeginOverlap(Capsule)
  (params (OverlappedComponent :type Primitive%20Component%20Object%20Reference) (OtherActor :type Actor%20Object%20Reference) (OtherComp :type Primitive%20Component%20Object%20Reference) (OtherBodyIndex :type Integer) (bFromSweep :type Boolean) (SweepResult :type Hit%20Result%20Structure%20%28by%20ref%29))
  (bind _as_bp_third_person_character (Variables|Reference|GetAs%20BP%20Third%20Person%20Character))
  ;[1 1 1] Voir si l'élément qui entre dans la collision de l'objet est le joueur
  (if (== OtherActor _as_bp_third_person_character)
    ;[1 1 1] Jouer le son du pick-up
    (Audio|PlaySound2D "/Game/Sons/Collectible/Son_Collectible_Cue.Son_Collectible_Cue" 1.0 1.0 0.0 0 0)
    (Utilities|FlowControl|Delay 0.2)
    (Audio|PlaySound2D "/Game/Sons/GainBatterie/GainBatterie_Cue.GainBatterie_Cue" 1.0 1.0 0.0 0 0)
    (Utilities|FlowControl|Sequence
      (:then_0
        ;[1 1 1] Détruit l'objet
        (Actor|DestroyActor))
      (:then_1
        ;[1 1 1] Remplir la jauge du joueur
        (Default|RecevoirBonusEnergie _as_bp_third_person_character (Variables|Energie|GetValeurEnergie))))))

(event Custom|Reverse
  (bind _scene (Variables|Default|GetScene))
  (bind _relativelocation (Variables|/Script/Engine.SceneComponent|GetRelativeLocation _scene))
  (bind _newtrack_0 (Timeline|LerpAnimationHautBas Reverse) ; Timeline
    (:Update
      ;[1 1 1] Modification de la position de l'objet
      (Transformation|SetRelativeLocation (Variables|Default|GetScene) (Math|Vector|MakeVector (.x _relativelocation) (.y _relativelocation) (Math|Float|Lerp 0.0 (+ (.z _relativelocation) (Variables|Default|GetIntervalle)) _newtrack_0)) false false))
    (:Finished
      ;[1 1 1] Changement de mode
      (if (Variables|Default|GetIsFromStart?)
        (Variables|Default|SetIsFromStart? false)
        (CallFunction|Reverse)
        (else
          (Variables|Default|SetIsFromStart? true)
          (CallFunction|Recommencer))))))

(event Custom|Recommencer
  (bind _scene (Variables|Default|GetScene))
  (bind _relativelocation (Variables|/Script/Engine.SceneComponent|GetRelativeLocation _scene))
  (bind _newtrack_0 (Timeline|LerpAnimationHautBas Play) ; Timeline
    (:Update
      ;[1 1 1] Modification de la position de l'objet
      (Transformation|SetRelativeLocation (Variables|Default|GetScene) (Math|Vector|MakeVector (.x _relativelocation) (.y _relativelocation) (Math|Float|Lerp 0.0 (+ (.z _relativelocation) (Variables|Default|GetIntervalle)) _newtrack_0)) false false))
    (:Finished
      ;[1 1 1] Changement de mode
      (if (Variables|Default|GetIsFromStart?)
        (Variables|Default|SetIsFromStart? false)
        (CallFunction|Reverse)
        (else
          (Variables|Default|SetIsFromStart? true)
          (CallFunction|Recommencer))))))

(event EventBeginPlay
  (bind _scene (Variables|Default|GetScene))
  (bind _relativelocation (Variables|/Script/Engine.SceneComponent|GetRelativeLocation _scene))
  ;[1 1 1] Prendre en référence le joueur
  (Utilities|FlowControl|Sequence
    (:then_0
      (bind _asbp_third_person_character (Utilities|Casting|CastToBP_ThirdPersonCharacter (Game|GetPlayerCharacter 0)))
      (Variables|Reference|SetAs%20BP%20Third%20Person%20Character _asbp_third_person_character))
    (:then_1
      (bind _newtrack_0 (Timeline|LerpAnimationHautBas Play) ; Timeline
        (:Update
          ;[1 1 1] Modification de la position de l'objet
          (Transformation|SetRelativeLocation (Variables|Default|GetScene) (Math|Vector|MakeVector (.x _relativelocation) (.y _relativelocation) (Math|Float|Lerp 0.0 (+ (.z _relativelocation) (Variables|Default|GetIntervalle)) _newtrack_0)) false false))
        (:Finished
          ;[1 1 1] Changement de mode
          (if (Variables|Default|GetIsFromStart?)
            (Variables|Default|SetIsFromStart? false)
            (CallFunction|Reverse)
            (else
              (Variables|Default|SetIsFromStart? true)
              (CallFunction|Recommencer))))))))

(fn ConstructionScript)