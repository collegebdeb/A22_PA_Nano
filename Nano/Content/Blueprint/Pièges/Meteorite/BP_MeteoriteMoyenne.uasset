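; Medium meteorite hazard that can be shot down and kills the player character on contact.
; On BeginPlay it caches the player and gives its RotatingMovement a random spin, printing the rate for debug.
; A Destruction event subtracts scaled shot damage from its hit points until depleted.
; Depletion or any hit triggers a shared Destroy event that spawns an explosion and removes the actor.
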(event Custom|Destroy
  ;[1 1 1] Fonction pour les multiples façons de détruire la météorite
  (Effects|SpawnEmitteratLocation "/Game/VFX/Mine_Explosion/P_Explosion.P_Explosion" (Transformation|GetWorldLocation (Variables|Default|GetMeteorite)) "0, 0, 0" "2.000000,2.000000,2.000000")
  (Actor|DestroyActor))

(event Collision|EventHit
  (params (MyComp :type Primitive%20Component%20Object%20Reference) (Other :type Actor%20Object%20Reference) (OtherComp :type Primitive%20Component%20Object%20Reference) (bSelfMoved :type Boolean) (HitLocation :type Vector :default "0, 0, 0") (HitNormal :type Vector :default "0, 0, 0") (NormalImpulse :type Vector :default "0, 0, 0") (Hit :type Hit%20Result%20Structure%20%28by%20ref%29))
  (bind _as_bp_third_person_character (Variables|Default|GetAs%20BP%20Third%20Person%20Character))
  ;[1 1 1] Détruire lorsque la météorite touche une surface
  (if (== Other _as_bp_third_person_character)
    (Default|Destroy _as_bp_third_person_character))
  (CallFunction|Destroy))

(event EventBeginPlay
  ;[1 1 1] Set la rotation aléatoire de la météorite
  (Utilities|FlowControl|Sequence
    (:then_0
      (bind _asbp_third_person_character (Utilities|Casting|CastToBP_ThirdPersonCharacter (Game|GetPlayerCharacter 0)))
      (Variables|Default|SetAs%20BP%20Third%20Person%20Character _asbp_third_person_character))
    (:then_1
      (bind _output_get (Variables|/Script/Engine.RotatingMovementComponent|SetRotationRate (Variables|Default|GetRotatingMovement) (Math|Rotator|MakeRotator (Math|Random|RandomFloatinRange 2.0 1e+01) (Math|Random|RandomFloatinRange 3.0 9.0) (Math|Random|RandomFloatinRange 2.0 5.0))))
      (Development|PrintString (Utilities|String|ToString(Rotator) _output_get)))))

(event EventDestruction
  (params (TirDegatParTir :type Integer) (DeltaTime :type Float%20%28double-precision%29))
  ;[1 1 1] Fonction pour calculer la santé de l'objet selon les tirs effectués
  (bind _output_get (Variables|Default|SetPV (- (Variables|Default|GetPV) (* TirDegatParTir (Variables|Default|GetEffectiveDamage)))))
  (if (<= _output_get 0)
    (CallFunction|Destroy)))

(fn ConstructionScript)