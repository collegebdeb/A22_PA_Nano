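; Destructible wall trap-folder actor that loses hit points (PV) through a Destruction event taking per-shot damage.
; BeginPlay creates dynamic materials for the wall and its crack decal, storing the decal's base emissive color.
; Tick interpolates the decal's emissive color and intensity from remaining PV.
; At depletion, it fires a rock particle burst and smash sound, removes the mesh, then destroys itself after a delay.
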(event EventBeginPlay
  (Utilities|FlowControl|Sequence
    (:then_0
      ;[1 1 1] Créer un matériel dynamique pour les murs destructibles
      (bind _returnvalue (Rendering|Material|CreateDynamicMaterialInstance "/Game/Megascans/Surfaces/Bunker_Concrete_Wall_tk3fbcgfw/M_Concrete.M_Concrete" "None" "None" :!class /Script/Engine.KismetMaterialLibrary))
      (bind _output_get (Variables|Default|SetConcrete _returnvalue))
      (Rendering|Material|SetMaterial (Variables|Default|GetMur) 0 _output_get))
    (:then_1
      ;[1 1 1] Créer un matériel dynamique pour les decals
      (bind _returnvalue_2 (Rendering|Material|CreateDynamicMaterialInstance "/Game/Megascans/Decals/Asphalt_Crack_umegfd0cw/MI_Asphalt_Crack_umegfd0cw_2K.MI_Asphalt_Crack_umegfd0cw_2K" "None" "None" :!class /Script/Engine.KismetMaterialLibrary))
      (bind _output_get_2 (Variables|Default|SetDecal _returnvalue_2))
      (bind _returnvalue_3 (Rendering|Material|GetVectorParameterValue _output_get_2 "EmissiveColor" :!class /Script/Engine.MaterialInstanceDynamic))
      (Variables|Default|SetColorBaseDecal _returnvalue_3)
      (bind _returnvalue_4 (Rendering|Material|GetScalarParameterValue _returnvalue_2 "Emmissive" :!class /Script/Engine.MaterialInstanceDynamic))
      (Development|PrintString (Utilities|String|ToString(Float) _returnvalue_4) true true "(R=1.000000,G=0.106016,B=0.016356,A=1.000000)")
      (Rendering|Components|Decal|SetDecalMaterial (Variables|Default|GetFissure) _returnvalue_2))))

(event EventTick
  (params (DeltaSeconds :type Float%20%28single-precision%29))
  (bind _returnvalue (* 1e+02 0.6))
  (bind _decal (Variables|Default|GetDecal))
  (bind _pv (Variables|HP|GetPV))
  (bind _returnvalue_2 (Math|Conversions|ToFloat(Integer) _pv))
  (bind _returnvalue_3 (/ _returnvalue_2 _returnvalue))
  (Rendering|Material|SetVectorParameterValue _decal "EmissiveColor" (Class|KismetMathLibrary|LinearColorLerpUsingHSV (Variables|Default|GetColorUpdate) (Variables|Default|GetColorBaseDecal) _returnvalue_3) :!class /Script/Engine.MaterialInstanceDynamic)
  (Rendering|Material|SetScalarParameterValue _decal "Emmissive" (Math|Float|Lerp (Variables|Default|GetNewVar_1) (+ (Variables|Default|GetNewVar_1) 4.0) _returnvalue_3) :!class /Script/Engine.MaterialInstanceDynamic))

(event EventDestruction
  (params (TirDegatParTir :type Integer) (DeltaTime :type Float%20%28double-precision%29))
  (bind _roches (Variables|Default|GetRoches))
  ;[1 1 1] Voir si les PVs du mur est égale à 0. Si oui, le détruit
  (Variables|HP|SetPV (- (Variables|HP|GetPV) (* TirDegatParTir 1)))
  (if (<= (- (Variables|HP|GetPV) (* TirDegatParTir 1)) 0)
    ;[1 1 1] Destruction du mur
    (Utilities|FlowControl|DoOnce false
      (:Completed
        (Components|Activation|Activate _roches false)
        (Effects|Components|ParticleSystem|SetFloatParameter _roches "SpawnRoche" 1.0)
        (Audio|PlaySound2D "/Game/Sons/MurDestructible/wall_smash_sound_effects__for_animations_1___mp3cut_net_.wall_smash_sound_effects__for_animations_1___mp3cut_net_" 0.7 0.7 0.0 0 0)
        (Components|DestroyComponent (Variables|Default|GetMur))
        (Utilities|FlowControl|Delay 3.0)
        (Effects|Components|ParticleSystem|SetFloatParameter (Variables|Default|GetRoches) "SpawnRoche" 0.0)
        (Actor|DestroyActor)))))

(fn ConstructionScript
  (Utilities|FlowControl|Sequence))

(fn Hit?)