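; BP_PiegeFeu is a fire trap effect that cycles its Niagara component on and off.
; Tick decrements a Seconds counter once per frame, so active time depends on frame rate despite the name.
; At zero, it sets particle velocity parameters to zero, then after a Delay resets the counter and restores them.
; The Blueprint has no overlap or damage logic.
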(event Collision|EventActorBeginOverlap
  (params (OtherActor :type Actor%20Object%20Reference)))

(event EventTick
  (params (DeltaSeconds :type Float%20%28single-precision%29))
  (bind _niagara (Variables|Default|GetNiagara))
  (bind _niagara_2 (Variables|Default|GetNiagara))
  (Variables|Default|SetSeconds (- (Variables|Default|GetSeconds) 1))
  (if (<= (Variables|Default|GetSeconds) 0)
    (Effects|Components|ParticleSystem|SetFloatParameter _niagara_2 "VelocityMin" 0.0)
    (Effects|Components|ParticleSystem|SetFloatParameter _niagara_2 "VelocityMax" 0.0)
    (Utilities|FlowControl|Delay 2e+01)
    (Variables|Default|SetSeconds 250)
    (Effects|Components|ParticleSystem|SetFloatParameter _niagara "VelocityMin" 1e+02)
    (Effects|Components|ParticleSystem|SetFloatParameter _niagara "VelocityMax" 4e+02)))

(fn ConstructionScript)