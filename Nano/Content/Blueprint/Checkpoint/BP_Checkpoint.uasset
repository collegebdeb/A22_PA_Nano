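; Checkpoint actor with sliding entry and exit doors that refills the player's energy and saves the respawn point.
; Overlapping the interior sets InCheckpoint and, once, updates the GameMode save, plays sounds and shows a notification widget.
; Two timelines lerp door Z offsets: OuvertureParPickUp opens the entry, then the exit if the player is inside, while OuverturePorte opens the exit for save loading.
; End-overlap events clear InCheckpoint and reverse the timelines to close doors.
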(event OnComponentBeginOverlap(InterieurCheckpoint)
  (params (OverlappedComponent :type Primitive%20Component%20Object%20Reference) (OtherActor :type Actor%20Object%20Reference) (OtherComp :type Primitive%20Component%20Object%20Reference) (OtherBodyIndex :type Integer) (bFromSweep :type Boolean) (SweepResult :type Hit%20Result%20Structure%20%28by%20ref%29))
  (bind _checkpoint (Variables|Checkpoint|GetCheckpoint))
  (bind _as_bp_third_person_character (Variables|Reference|GetAs%20BP%20Third%20Person%20Character))
  ;[0.9391 1 0] Lorsque le joueur entre dans la zone de sauvegarde
  ;;[1 1 1] Si il y a une collision avec le personnage, continue le code
  (if (== OtherActor (Variables|Reference|GetAs%20BP%20Third%20Person%20Character))
    ;;[1 1 1] Change les varaiables lorsque le joueur overlap avec la triggerbox
    (Variables|/Game/ThirdPerson/Blueprints/BP_ThirdPersonCharacter.BP_ThirdPersonCharacter_C|SetEnergieActuelle _as_bp_third_person_character (Variables|/Game/ThirdPerson/Blueprints/BP_ThirdPersonCharacter.BP_ThirdPersonCharacter_C|GetEnergieLimite _as_bp_third_person_character))
    (Variables|/Game/ThirdPerson/Blueprints/BP_ThirdPersonCharacter.BP_ThirdPersonCharacter_C|SetIn%20Checkpoint? _as_bp_third_person_character true)
    (Utilities|FlowControl|DoOnce false ; Fait une seule fois (Optimisation et empêche la possibilité de bug)
      (:Completed
        ;;[1 1 1] Fait une sauvegarde des variables pour le fichier Save
        (Default|UpdateApparitionSave (Variables|Reference|GetAs%20BP%20Nano%20Game%20Mode) _checkpoint (Utilities|Array|Get(acopy) (Variables|/Script/Engine.Actor|GetTags _checkpoint)) true)
        ;;[1 1 1] Lorsqu'il entre dans le checkpoint, un son joue
        (Audio|PlaySound2D 0 1.0 1.0 0.0 0 0)
        (Utilities|FlowControl|Delay 0.4)
        (Audio|PlaySound2D 0 1.0 1.0 0.0 0 0)
        ;[1 0 0.05503] Apparition de la notification pour le checkpoint
        (bind _returnvalue (UserInterface|CreateWidget "/Game/Blueprint/HUD/HUD_Gameplay/NotificationCheckpoint.NotificationCheckpoint_C"))
        (bind _output_get (Variables|Reference|SetApparitionNotification _returnvalue))
        (UserInterface|Viewport|AddtoViewport _output_get 0)))))

(event OnComponentEndOverlap(InterieurCheckpoint)
  (params (OverlappedComponent :type Primitive%20Component%20Object%20Reference) (OtherActor :type Actor%20Object%20Reference) (OtherComp :type Primitive%20Component%20Object%20Reference) (OtherBodyIndex :type Integer))
  (bind _as_bp_third_person_character (Variables|Reference|GetAs%20BP%20Third%20Person%20Character))
  ;[1 1 1] Lorsque le joueur quitte la zone, les propulseurs regagnent la possibilité d'épuiser de l'énergie (Inverse l'animation de la porte droite aussi)
  (if (== OtherActor _as_bp_third_person_character)
    (Variables|/Game/ThirdPerson/Blueprints/BP_ThirdPersonCharacter.BP_ThirdPersonCharacter_C|SetIn%20Checkpoint? _as_bp_third_person_character false)))

(event OnComponentEndOverlap(CollisionOuvrirCheckpoint)
  (params (OverlappedComponent :type Primitive%20Component%20Object%20Reference) (OtherActor :type Actor%20Object%20Reference) (OtherComp :type Primitive%20Component%20Object%20Reference) (OtherBodyIndex :type Integer))
  ;[0 0 0] Lorsque le joueur entre dans cette collision
  ;;[1 1 1] N'est plu en overlap avec la boîte de collision
  (if (== OtherActor (Variables|Reference|GetAs%20BP%20Third%20Person%20Character))
    (CallFunction|FermeturePorte)))

(event OnComponentEndOverlap(Box)
  (params (OverlappedComponent :type Primitive%20Component%20Object%20Reference) (OtherActor :type Actor%20Object%20Reference) (OtherComp :type Primitive%20Component%20Object%20Reference) (OtherBodyIndex :type Integer))
  (bind _as_bp_third_person_character (Variables|Reference|GetAs%20BP%20Third%20Person%20Character))
  (bind _relativepositionportedroite (Variables|Animation|GetRelativePositionPorteDroite))
  ;[1 1 1] Referme la porte si le joueur sort complètement à l'extérieur du checkpoint
  (if (and (== OtherActor _as_bp_third_person_character) (not (Variables|/Game/ThirdPerson/Blueprints/BP_ThirdPersonCharacter.BP_ThirdPersonCharacter_C|GetIn%20Checkpoint? _as_bp_third_person_character)))
    (Utilities|FlowControl|Delay 0.2)
    ;[1 0.4863 0] Si le joueur est dans le checkpoint, joue l'animation qui ouvre la porte droite
    (bind _opacity_animation (Timeline|Opacity%20Mask%20%28Porte%20de%20Sortie%29 Reverse)
      (:Update
        ;;[1 1 1] Déplacement de la porte selon l'événement
        (Transformation|SetRelativeLocation (Variables|Default|GetPorteFin) (Math|Vector|MakeVector (.x _relativepositionportedroite) (.y _relativepositionportedroite) (+ (.z _relativepositionportedroite) (Math|Float|Lerp 0.0 (Variables|Animation|GetDeplacementPorte) _opacity_animation))) false false)))))

(event Custom|FermeturePorte
  (bind _relativepositionportegauche (Variables|Animation|GetRelativePositionPorteGauche))
  (bind _relativepositionportedroite (Variables|Animation|GetRelativePositionPorteDroite))
  (bind _as_bp_third_person_character (Variables|Reference|GetAs%20BP%20Third%20Person%20Character))
  ;[0 0 0] Lorsque le joueur entre dans cette collision
  ;;[0 0 0] Ajoute un delay à la fermeture de la porte
  (Utilities|FlowControl|Delay 0.5)
  ;[0 0.9636 1] Timeline (Opacity) pour fermeture et ouverture de la porte pour entrer
  (bind _opacity_animation (Timeline|AnimationTransform Reverse)
    (:Update
      ;[0.2457 0 1] Créer l'animation de la porte gauche (ouverture ou fermeture selon si le personnage est en dehors ou à l'intérieur du checkpoint)
      (Transformation|SetRelativeLocation (Variables|Default|GetPorteAvant) (Math|Vector|MakeVector (.x _relativepositionportegauche) (.y _relativepositionportegauche) (+ (.z _relativepositionportegauche) (Math|Float|Lerp 0.0 (Variables|Animation|GetDeplacementPorte) _opacity_animation))) false false))
    (:Finished
      ;[1 0.4863 0] Si le personnage est valide (Débug)
      (Utilities|IsValid _as_bp_third_person_character
        (:Is%20Valid
          ;[1 0.4863 0] Si le joueur est dans le checkpoint, joue l'animation qui ouvre la porte droite
          (if (Variables|/Game/ThirdPerson/Blueprints/BP_ThirdPersonCharacter.BP_ThirdPersonCharacter_C|GetIn%20Checkpoint? _as_bp_third_person_character)
            (Utilities|FlowControl|Delay 0.5)
            (bind _opacity_animation_2 (Timeline|Opacity%20Mask%20%28Porte%20de%20Sortie%29 Play)
              (:Update
                ;;[1 1 1] Déplacement de la porte selon l'événement
                (Transformation|SetRelativeLocation (Variables|Default|GetPorteFin) (Math|Vector|MakeVector (.x _relativepositionportedroite) (.y _relativepositionportedroite) (+ (.z _relativepositionportedroite) (Math|Float|Lerp 0.0 (Variables|Animation|GetDeplacementPorte) _opacity_animation_2))) false false)))))))))

(event Custom|OuvertureParPickUp
  (bind _relativepositionportegauche (Variables|Animation|GetRelativePositionPorteGauche))
  (bind _relativepositionportedroite (Variables|Animation|GetRelativePositionPorteDroite))
  (bind _as_bp_third_person_character (Variables|Reference|GetAs%20BP%20Third%20Person%20Character))
  ;[0 0 0] Lorsque le joueur entre dans cette collision
  ;;[1 1 1] En overlap avec la boîte de collision
  (Utilities|FlowControl|DoOnce false ; Le fait une seule fois. Si il en sort, reset la condition du node
    (:Completed
      ;[0 0.9636 1] Timeline (Opacity) pour fermeture et ouverture de la porte pour entrer
      (bind _opacity_animation (Timeline|AnimationTransform Play)
        (:Update
          ;[0.2457 0 1] Créer l'animation de la porte gauche (ouverture ou fermeture selon si le personnage est en dehors ou à l'intérieur du checkpoint)
          (Transformation|SetRelativeLocation (Variables|Default|GetPorteAvant) (Math|Vector|MakeVector (.x _relativepositionportegauche) (.y _relativepositionportegauche) (+ (.z _relativepositionportegauche) (Math|Float|Lerp 0.0 (Variables|Animation|GetDeplacementPorte) _opacity_animation))) false false))
        (:Finished
          ;[1 0.4863 0] Si le personnage est valide (Débug)
          (Utilities|IsValid _as_bp_third_person_character
            (:Is%20Valid
              ;[1 0.4863 0] Si le joueur est dans le checkpoint, joue l'animation qui ouvre la porte droite
              (if (Variables|/Game/ThirdPerson/Blueprints/BP_ThirdPersonCharacter.BP_ThirdPersonCharacter_C|GetIn%20Checkpoint? _as_bp_third_person_character)
                (Utilities|FlowControl|Delay 0.5)
                (bind _opacity_animation_2 (Timeline|Opacity%20Mask%20%28Porte%20de%20Sortie%29 Play)
                  (:Update
                    ;;[1 1 1] Déplacement de la porte selon l'événement
                    (Transformation|SetRelativeLocation (Variables|Default|GetPorteFin) (Math|Vector|MakeVector (.x _relativepositionportedroite) (.y _relativepositionportedroite) (+ (.z _relativepositionportedroite) (Math|Float|Lerp 0.0 (Variables|Animation|GetDeplacementPorte) _opacity_animation_2))) false false)))))))))))

(event EventOuverturePorte
  (bind _relativepositionportedroite (Variables|Animation|GetRelativePositionPorteDroite))
  ;[1 0.4863 0] Si le joueur est dans le checkpoint, joue l'animation qui ouvre la porte droite
  ;;[1 1 1] Sauvegarde (Lancement du jeu)
  (Utilities|FlowControl|Delay 0.5)
  (bind _opacity_animation (Timeline|Opacity%20Mask%20%28Porte%20de%20Sortie%29 Play)
    (:Update
      ;;[1 1 1] Déplacement de la porte selon l'événement
      (Transformation|SetRelativeLocation (Variables|Default|GetPorteFin) (Math|Vector|MakeVector (.x _relativepositionportedroite) (.y _relativepositionportedroite) (+ (.z _relativepositionportedroite) (Math|Float|Lerp 0.0 (Variables|Animation|GetDeplacementPorte) _opacity_animation))) false false))))

(event EventBeginPlay
  (Utilities|FlowControl|Sequence
    (:then_0
      ;[0 1 0.4047] Sauvegarder le personnage
      (bind _asbp_third_person_character (Utilities|Casting|CastToBP_ThirdPersonCharacter (Game|GetPlayerCharacter 0)))
      (Variables|Reference|SetAs%20BP%20Third%20Person%20Character _asbp_third_person_character))
    (:then_1
      ;[1 0.3 0.7262] Sauvegarder Game Mode
      (bind _asbp_nano_game_mode (Utilities|Casting|CastToBP_Nano_GameMode (Game|GetGameMode)))
      (Variables|Reference|SetAs%20BP%20Nano%20Game%20Mode _asbp_nano_game_mode))
    (:then_2
      ;[1 0 0] Prendre la valeur initiale de la position des portes dans le monde et sauvegarder dans une variable
      ;;[1 1 1] Avoir la position de la porte gauche
      (Variables|Animation|SetRelativePositionPorteGauche (Variables|/Script/Engine.SceneComponent|GetRelativeLocation (Variables|Default|GetPorteAvant))))
    (:then_3
      ;;[1 1 1] Avoir la position de la porte droite
      (Variables|Animation|SetRelativePositionPorteDroite (Variables|/Script/Engine.SceneComponent|GetRelativeLocation (Variables|Default|GetPorteFin))))))

(fn ConstructionScript)