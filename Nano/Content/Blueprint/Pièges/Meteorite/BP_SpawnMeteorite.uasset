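; Meteorite spawner trap that continuously spawns actors of a configurable class at its sphere's location, using its arrow's relative rotation.
; From BeginPlay, a self-calling delayed event spawns each one, stores it in an array and adds a projectile movement component with a set max speed.
; A fast looping timer caps the count by destroying the oldest, provided it is valid and casts to BP_MeteoritePetite.
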(event Custom|SpawnAnother
  (bind _array_spawnactor (Variables|Default|GetArray_SpawnActor))
  (bind _returnvalue (Game|SpawnActorfromClass (Variables|Default|GetClassMeteorite) (Math|Transform|MakeTransform (Transformation|GetWorldLocation (Variables|Default|GetSphere)) (Variables|/Script/Engine.SceneComponent|GetRelativeRotation (Variables|Default|GetArrow)) "1.000000,1.000000,1.000000") "Undefined" 0 0))
  (bind _output_get (Variables|Default|SetSpawnActor _returnvalue))
  (bind _returnvalue_2 (Utilities|Array|Add _array_spawnactor _output_get))
  (bind _returnvalue_3 (AddComponent|AddProjectileMovementComponent (Utilities|Array|Get(acopy) _array_spawnactor _returnvalue_2)))
  (bind _output_get_2 (Variables|Default|SetNewVar_1 _returnvalue_3))
  (Variables|/Script/Engine.ProjectileMovementComponent|SetMaxSpeed _output_get_2 (Variables|Default|GetVelocityProjectile))
  (Utilities|FlowControl|Delay (Variables|Default|GetTempsEntreApparition))
  (CallFunction|SpawnAnother))

(event Custom|VoirSiLimiteAtteint
  (bind _array_spawnactor (Variables|Default|GetArray_SpawnActor))
  (bind _returnvalue (Utilities|Array|Length _array_spawnactor))
  (bind _output (Utilities|Array|Get(acopy) _array_spawnactor))
  (if (> _returnvalue (Variables|Default|GetNombrePossibleMeteorite))
    (Utilities|IsValid _output
      (:Is%20Valid
        (bind _asbp_meteorite_petite (Utilities|Casting|CastToBP_MeteoritePetite _output))
        (Default|Destroy _asbp_meteorite_petite)
        (Utilities|Array|RemoveIndex _array_spawnactor)
        (Development|PrintString (Utilities|String|ToString(Integer) _returnvalue))))))

(event EventBeginPlay
  (bind _array_spawnactor (Variables|Default|GetArray_SpawnActor))
  (Utilities|Time|SetTimerbyEvent (delegate Custom|VoirSiLimiteAtteint) 0.1 true)
  (bind _returnvalue (Game|SpawnActorfromClass (Variables|Default|GetClassMeteorite) (Math|Transform|MakeTransform (Transformation|GetWorldLocation (Variables|Default|GetSphere)) (Variables|/Script/Engine.SceneComponent|GetRelativeRotation (Variables|Default|GetArrow)) "1.000000,1.000000,1.000000") "Undefined" 0 0))
  (bind _output_get (Variables|Default|SetSpawnActor _returnvalue))
  (bind _returnvalue_2 (Utilities|Array|Add _array_spawnactor _output_get))
  (bind _returnvalue_3 (AddComponent|AddProjectileMovementComponent (Utilities|Array|Get(acopy) _array_spawnactor _returnvalue_2)))
  (bind _output_get_2 (Variables|Default|SetNewVar_1 _returnvalue_3))
  (Variables|/Script/Engine.ProjectileMovementComponent|SetMaxSpeed _output_get_2 (Variables|Default|GetVelocityProjectile))
  (Utilities|FlowControl|Delay (Variables|Default|GetTempsEntreApparition))
  (CallFunction|SpawnAnother))

(fn ConstructionScript)

(fn ParametreMeteorite
  (params (ProjectileComponent :type Projectile%20Movement%20Component%20Object%20Reference)))