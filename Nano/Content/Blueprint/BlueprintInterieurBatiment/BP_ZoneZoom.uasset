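; BP_ZoneZoom is a trigger volume that changes the third-person camera's boom length as the player enters or leaves it.
; BeginPlay caches the character and its starting arm length.
; Box overlaps drive a timeline lerping that length to a target and back; InZoom and an actor check only select the playback mode, so other actors also trigger it.
; The construction script sizes the box from ScaleX and ScaleZ.
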(event OnComponentBeginOverlap(Box)
  (params (OverlappedComponent :type Primitive%20Component%20Object%20Reference) (OtherActor :type Actor%20Object%20Reference) (OtherComp :type Primitive%20Component%20Object%20Reference) (OtherBodyIndex :type Integer) (bFromSweep :type Boolean) (SweepResult :type Hit%20Result%20Structure%20%28by%20ref%29))
  (if (and (== OtherActor (Variables|Default|GetThirdPersonCharacter)) (Variables|Default|GetInZoom?))
    (bind _newtrack_0 (Timeline|Lerp Play)
      (:Update
        (Variables|/Script/Engine.SpringArmComponent|SetTargetArmLength (Variables|/Game/ThirdPerson/Blueprints/BP_ThirdPersonCharacter.BP_ThirdPersonCharacter_C|GetCameraBoom (Variables|Default|GetThirdPersonCharacter)) (Math|Float|Lerp (Variables|Default|GetTarget%20Arm%20Length%20Base) (Variables|Default|GetTarget%20Arm%20Length%20Final) _newtrack_0))))
    (else
      (Timeline|Lerp PlayFromStart))))

(event OnComponentEndOverlap(Box)
  (params (OverlappedComponent :type Primitive%20Component%20Object%20Reference) (OtherActor :type Actor%20Object%20Reference) (OtherComp :type Primitive%20Component%20Object%20Reference) (OtherBodyIndex :type Integer))
  (if (and (== OtherActor (Variables|Default|GetThirdPersonCharacter)) (Variables|Default|GetInZoom?))
    (Utilities|FlowControl|Delay 0.1)
    (bind _newtrack_0 (Timeline|Lerp ReverseFromEnd)
      (:Update
        (Variables|/Script/Engine.SpringArmComponent|SetTargetArmLength (Variables|/Game/ThirdPerson/Blueprints/BP_ThirdPersonCharacter.BP_ThirdPersonCharacter_C|GetCameraBoom (Variables|Default|GetThirdPersonCharacter)) (Math|Float|Lerp (Variables|Default|GetTarget%20Arm%20Length%20Base) (Variables|Default|GetTarget%20Arm%20Length%20Final) _newtrack_0))))
    (else
      (Timeline|Lerp Reverse))))

(event EventBeginPlay
  (Utilities|FlowControl|Sequence
    (:then_0
      (bind _asbp_third_person_character (Utilities|Casting|CastToBP_ThirdPersonCharacter (Game|GetPlayerCharacter 0)))
      (Variables|Default|SetThirdPersonCharacter _asbp_third_person_character)
      (Variables|Default|SetTarget%20Arm%20Length%20Base (Variables|/Script/Engine.SpringArmComponent|GetTargetArmLength (Variables|/Game/ThirdPerson/Blueprints/BP_ThirdPersonCharacter.BP_ThirdPersonCharacter_C|GetCameraBoom (Variables|Default|GetThirdPersonCharacter)))))))

(fn ConstructionScript
  (Utilities|FlowControl|Sequence
    (:then_0
      (Transformation|SetWorldScale3D (Variables|Default|GetBox) (Math|Vector|MakeVector (Variables|Scale|GetScaleX) 8.0 (Variables|Scale|GetScaleZ))))))