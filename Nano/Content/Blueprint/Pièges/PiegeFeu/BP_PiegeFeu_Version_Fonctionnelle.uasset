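; Fire trap that periodically switches its flames on and off and kills the player character on contact.
; A Tick-driven countdown turns the trap off, waits through a Delay, then reactivates it and resets the timer.
; The toggle functions set Niagara velocity parameters and the Box collision together, so the kill zone follows the flames.
; Box overlap with BP_ThirdPersonCharacter calls its Mort function.
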(event OnComponentBeginOverlap(Box)
  (params (OverlappedComponent :type Primitive%20Component%20Object%20Reference) (OtherActor :type Actor%20Object%20Reference) (OtherComp :type Primitive%20Component%20Object%20Reference) (OtherBodyIndex :type Integer) (bFromSweep :type Boolean) (SweepResult :type Hit%20Result%20Structure%20%28by%20ref%29))
  ;[1 1 1] Mort du personnage lorsqu'il touche les flammes
  (bind _asbp_third_person_character (Utilities|Casting|CastToBP_ThirdPersonCharacter OtherActor))
  (bind _output_get (Variables|Default|SetAs%20BP%20Third%20Person%20Character _asbp_third_person_character))
  (Default|Mort _output_get))

(event Collision|EventActorBeginOverlap
  (params (OtherActor :type Actor%20Object%20Reference)))

(event EventTick
  (params (DeltaSeconds :type Float%20%28single-precision%29))
  (bind _output_get (Variables|Default|SetTimer (- (Variables|Default|GetTimer) DeltaSeconds)))
  (if (<= _output_get 0.0)
    (CallFunction|DésactiverPiege)
    (Utilities|FlowControl|Delay 5.0)
    (CallFunction|ActiverPiege)
    (Variables|Default|SetTimer 6.0)))

(fn ConstructionScript)

(fn ActiverPiege
  (bind _niagara (Variables|Default|GetNiagara))
  (Effects|Components|ParticleSystem|SetFloatParameter _niagara "VelocityMin" 1e+02)
  (Effects|Components|ParticleSystem|SetFloatParameter _niagara "VelocityMax" 3e+02)
  (Collision|SetCollisionEnabled (Variables|Default|GetBox) "QueryAndPhysics")
  (return))

(fn DésactiverPiege
  (bind _niagara (Variables|Default|GetNiagara))
  (Effects|Components|ParticleSystem|SetFloatParameter _niagara "VelocityMin" 0.0)
  (Effects|Components|ParticleSystem|SetFloatParameter _niagara "VelocityMax" 0.0)
  (Collision|SetCollisionEnabled (Variables|Default|GetBox) "NoCollision")
  (return))