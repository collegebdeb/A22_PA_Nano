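; Midpoint checkpoint actor that saves the player's respawn point when the character enters its trigger volume.
; BeginPlay caches the ThirdPerson character and Nano game mode.
; The first overlap by the player passes the Checkpoint reference and its first tag to the game mode's save update, via a DoOnce.
; It then plays a sound and briefly shows a checkpoint notification widget before removing it.
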(event OnComponentBeginOverlap(InterieurCheckpoint)
  (params (OverlappedComponent :type Primitive%20Component%20Object%20Reference) (OtherActor :type Actor%20Object%20Reference) (OtherComp :type Primitive%20Component%20Object%20Reference) (OtherBodyIndex :type Integer) (bFromSweep :type Boolean) (SweepResult :type Hit%20Result%20Structure%20%28by%20ref%29))
  (bind _checkpoint (Variables|Checkpoint|GetCheckpoint))
  ;[0.9391 1 0] Lorsque le joueur entre dans la zone de sauvegarde
  ;;[1 1 1] Si il y a une collision avec le personnage, continue le code
  (if (== OtherActor (Variables|Reference|GetAs%20BP%20Third%20Person%20Character))
    (Utilities|FlowControl|DoOnce false ; Fait une seule fois (Optimisation et empêche la possibilité de bug)
      (:Completed
        ;;[1 1 1] Fait une sauvegarde des variables pour le fichier Save
        (Default|UpdateApparitionSave (Variables|Reference|GetAs%20BP%20Nano%20Game%20Mode) _checkpoint (Utilities|Array|Get(acopy) (Variables|/Script/Engine.Actor|GetTags _checkpoint)))
        ;;[1 1 1] Lorsqu'il entre dans le checkpoint, un son joue
        (Audio|PlaySound2D "/Game/Sons/Checkpoint_Sound_Effect.Checkpoint_Sound_Effect" 1.0 1.0 0.0 0 0)
        (Utilities|FlowControl|Delay 0.2)
        ;[1 0 0.05503] Apparition de la notification pour le checkpoint
        (bind _returnvalue (UserInterface|CreateWidget "/Game/Blueprint/HUD/HUD_Gameplay/NotificationCheckpoint.NotificationCheckpoint_C"))
        (bind _output_get (Variables|Default|SetApparitionNotification _returnvalue))
        (UserInterface|Viewport|AddtoViewport _output_get 0)
        (Utilities|FlowControl|Delay 2.0)
        (Widget|RemovefromParent (Variables|Default|GetApparitionNotification))))))

(event EventBeginPlay
  (Utilities|FlowControl|Sequence
    (:then_0
      ;[0 1 0.4047] Sauvegarder le personnage
      (bind _asbp_third_person_character (Utilities|Casting|CastToBP_ThirdPersonCharacter (Game|GetPlayerCharacter 0)))
      (Variables|Reference|SetAs%20BP%20Third%20Person%20Character _asbp_third_person_character))
    (:then_1
      ;[1 0.3 0.7262] Sauvegarder Game Mode
      (bind _asbp_nano_game_mode (Utilities|Casting|CastToBP_Nano_GameMode (Game|GetGameMode)))
      (Variables|Reference|SetAs%20BP%20Nano%20Game%20Mode _asbp_nano_game_mode))))

(fn ConstructionScript)